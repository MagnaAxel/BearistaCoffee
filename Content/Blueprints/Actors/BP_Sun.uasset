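; BP_Sun is a light actor that moves the sun from morning to evening over the coffee game's playing day.
; A Progress value blends rotation and light color between morning and evening settings, applied in the construction script and through SetProgress.
; BeginPlay registers with the game state's playing-day event, and BindDay converts the day timer to progress, rescheduling each tick while that timer is active.
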(event `self.ReceiveBeginPlay`
  (bind _output_get (set `self.GSB` (`/Game/Blueprints/Systems/FL_System.GetGSB_BearistaCoffee`)))
  (add `/Game/Blueprints/Systems/GSB_BearistaCoffee.PlayingDay` _output_get (`|CreateDelegate` :!event `BindDay`)))

(fn `ApplyProgress`
  (`self.K2_SetActorRotation` (`KismetMathLibrary.RLerp` (`self.MorningRotator`) (`self.EveningRotator`) (`self.Progress`) true))
  (`LightComponent.SetLightColor` (`self.LightComponent`) (`KismetMathLibrary.LinearColorLerp` (`self.MorningColor`) (`self.EveningColor`) (`self.Progress`)) true))

(fn `BindDay`
  (bind _daytimer (`/Game/Blueprints/Systems/GSB_BearistaCoffee.GetDayTimer` (`self.GSB`)))
  (if (`KismetSystemLibrary.K2_IsTimerActiveHandle` _daytimer)
    (bind _percent (`/Game/Blueprints/FL_Common.TimerHandleToPercent` _daytimer))
    (`self.SetProgress` _percent)
    (`KismetSystemLibrary.K2_SetTimerForNextTickDelegate` (`|CreateDelegate` :!event `BindDay`))))

(fn `SetProgress`
  (params (Progress :type "Float (double-precision)"))
  (set `self.Progress` Progress)
  (`self.ApplyProgress`))

(fn `UserConstructionScript`
  (`self.ApplyProgress`))