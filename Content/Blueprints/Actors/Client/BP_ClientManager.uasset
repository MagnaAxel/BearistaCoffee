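; Client manager actor for a coffee shop game that sends customers in while the day is being played.
; Day events from the AC_Door component start and stop a self-rearming timer on a fixed one-second delay.
; Each tick shuffles the existing client pool and makes the first unnamed client enter, with a random EN_Client name not already in use.
; The popularity-based spawn delay is present but unconnected.
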(event `self.ReceiveBeginPlay`
  (bind _returnvalue (`self.GetComponentByClass` (`self.Day`) "/Game/Blueprints/Actors/Interactives/Instances/AC_Door.AC_Door_C"))
  (add `/Game/Blueprints/Actors/Interactives/Instances/AC_Door.PlayingDay` _returnvalue (delegate `PlayingDay_Event`))
  (add `/Game/Blueprints/Actors/Interactives/Instances/AC_Door.PlayedDay` _returnvalue (delegate `PlayedDay_Event`)))

(event `PlayingDay_Event`
  (`self.ClientLoop`))

(event `PlayedDay_Event`
  (`KismetSystemLibrary.K2_ClearAndInvalidateTimerHandle` (`self.ClientLoopTimer`)))

(event `ClientLoop`
  (bind _returnvalue (`KismetSystemLibrary.K2_SetTimerDelegate` (delegate `ClientLoop_Event`) 1.0))
  (set `self.ClientLoopTimer` _returnvalue))

(event `ClientLoop_Event`
  (`self.LaunchClient`)
  (`self.ClientLoop`))

(fn `LaunchClient`
  (returns (Success :type Boolean))
  (`KismetArrayLibrary.Array_Shuffle` (`self.Clients`))
  (for _array_element (`self.Clients`)
    (if (== (`/Game/Blueprints/Actors/Client/BP_Client.GetName` _array_element) 0)
      (`/Game/Blueprints/Actors/Client/BP_Client.SetName` _array_element (`self.RandomName`))
      (`/Game/Blueprints/Actors/Client/BP_Client.Enter` _array_element)
      (return true)))
  (return false))

(fn `RandomName`
  (returns (Name :type "/Game/DataBase/Client/EN_Client Enum"))
  (locals (LocalNames :type "Array of /Game/DataBase/Client/EN_Client Enum"))
  (`|ExecutionSequence`
    (:`then_0`
      (bind _enumvalue (foreach `/Game/DataBase/Client/EN_Client` false)
        (:`LoopBody`
          (`KismetArrayLibrary.Array_Add` (`local.LocalNames`) _enumvalue))))
    (:`then_1`
      (`KismetArrayLibrary.Array_RemoveItem` (`local.LocalNames`) "NewEnumerator0"))
    (:`then_2`
      (for _array_element (`self.Clients`)
        (`KismetArrayLibrary.Array_RemoveItem` (`local.LocalNames`) (`/Game/Blueprints/Actors/Client/BP_Client.GetName` _array_element))))
    (:`then_3`
      (return (`KismetArrayLibrary.Array_Random` (`local.LocalNames`))))))

(fn `UserConstructionScript`)