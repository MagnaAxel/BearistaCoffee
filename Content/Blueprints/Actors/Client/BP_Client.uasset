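; Client actor for the coffee shop game that walks to its Spot, orders a random drink and pastry, then leaves.
; Timer-driven per-tick loops move it along the Spot's spline, with mesh and animation loaded from its Name's client data.
; While waiting on a pausable, difficulty-based timer, slot changes are checked against the order.
; A match is eaten and rewarded with popularity, pawies, affinity and story progression, while a timeout is punished.
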(event `self.ReceiveBeginPlay`
  (message `/Game/Blueprints/Widgets/Interfaces/IN_ActorWidget.BindActor` (`WidgetComponent.GetWidget` (`self.WI_Client`)) self))

(event `Leave`
  (bind _returnvalue (`KismetSystemLibrary.K2_SetTimerDelegate` (delegate `Leave_Event`) (/ (`SplineComponent.GetSplineLength` (`self.GetComponentByClass` (`self.Spot`) "/Script/Engine.SplineComponent")) (`self.WalkSpeed`))))
  (set `self.WalkTimer` _returnvalue)
  (`|ExecutionSequence`
    (:`then_0`
      (`self.K2_SetActorTransform` (`/Game/Blueprints/FL_Common.GetSplineTransformAt` (`self.GetComponentByClass` (`self.Spot`) "/Script/Engine.SplineComponent") (`/Game/Blueprints/FL_Common.TimerHandleToPercent` (`self.WalkTimer`))) :!label _label)
      (`KismetSystemLibrary.DelayUntilNextTick`)
      (if (`KismetSystemLibrary.K2_IsValidTimerHandle` (`self.WalkTimer`))
        (goto _label)))
    (:`then_1`)))

(event `Leave_Event`
  (`KismetSystemLibrary.K2_ClearAndInvalidateTimerHandle` (`self.WalkTimer`))
  (`self.SetName` "NewEnumerator0"))

(event `Enter`
  (bind _returnvalue (`self.GetComponentByClass` (`self.Spot`) "/Script/Engine.SplineComponent"))
  (bind _returnvalue_2 (`KismetSystemLibrary.K2_SetTimerDelegate` (delegate `Enter_Event`) (/ (`SplineComponent.GetSplineLength` (`self.GetComponentByClass` (`self.Spot`) "/Script/Engine.SplineComponent")) (`self.WalkSpeed`))))
  (set `self.WalkTimer` _returnvalue_2)
  (`|ExecutionSequence`
    (:`then_0`
      (`self.K2_SetActorTransform` (`KismetMathLibrary.MakeTransform` (.location (`/Game/Blueprints/FL_Common.GetSplineTransformAt` _returnvalue (`/Game/Blueprints/FL_Common.TimerHandleToPercent` (`self.WalkTimer`) true))) (`KismetMathLibrary.ComposeRotators` (.rotation (`/Game/Blueprints/FL_Common.GetSplineTransformAt` _returnvalue (`/Game/Blueprints/FL_Common.TimerHandleToPercent` (`self.WalkTimer`) true))) (struct :`Yaw` 180.0)) (.scale (`/Game/Blueprints/FL_Common.GetSplineTransformAt` _returnvalue (`/Game/Blueprints/FL_Common.TimerHandleToPercent` (`self.WalkTimer`) true)))) :!label _label_2)
      (`KismetSystemLibrary.DelayUntilNextTick`)
      (if (`KismetSystemLibrary.K2_IsValidTimerHandle` (`self.WalkTimer`))
        (goto _label_2)
        (else
          (`self.K2_SetActorTransform` (`KismetMathLibrary.MakeTransform` (.location (`/Game/Blueprints/FL_Common.GetSplineTransformAt` _returnvalue)) (`KismetMathLibrary.ComposeRotators` (.rotation (`/Game/Blueprints/FL_Common.GetSplineTransformAt` _returnvalue)) (struct :`Yaw` 180.0)) (.scale (`/Game/Blueprints/FL_Common.GetSplineTransformAt` _returnvalue)))))))
    (:`then_1`)))

(event `Enter_Event`
  (`KismetSystemLibrary.K2_ClearAndInvalidateTimerHandle` (`self.WalkTimer`))
  (`self.Wait`))

(event `Wait`
  (bind (_drink _pastrie) (`self.RandomOrder`))
  (bind _returnvalue (`self.GetComponentByClass` (`self.Spot`) "/Game/Blueprints/Actors/Slots/AC_Slot.AC_Slot_C"))
  (`|ExecutionSequence`
    (:`then_0`
      (`self.SetOrder` _drink _pastrie))
    (:`then_1`
      (bind _returnvalue_2 (`KismetSystemLibrary.K2_SetTimerDelegate` (delegate `Wait_Event`) (`self.GetOrderDelay`)))
      (set `self.WaitTimer` _returnvalue_2)
      (`self.ApplyPaused`)
      (`self.Waiting`))
    (:`then_2`
      (add `/Game/Blueprints/Actors/Slots/AC_Slot.Slotted` _returnvalue (delegate `Slot_Event`))
      (add `/Game/Blueprints/Actors/Slots/AC_Slot.Unslotted` _returnvalue (delegate `Slot_Event`)))))

(event `Wait_Event`
  (bind _ns_grumble (`self.NS_Grumble`))
  (`self.EndOfWait` (delegate `Slot_Event`))
  (`self.Punish`)
  (`self.Leave`)
  (`NiagaraComponent.ResetSystem` _ns_grumble)
  (`ActorComponent.Activate` _ns_grumble false))

(event `Slot_Event`
  (params (Actor :type "Actor Object Reference"))
  (bind _tool (`/Game/Blueprints/Actors/Slots/AC_Slot.GetTool` (`self.GetComponentByClass` (`self.Spot`) "/Game/Blueprints/Actors/Slots/AC_Slot.AC_Slot_C") (`self.CupSlot`)))
  (if (`self.ServiceMatchOrder`)
    (`self.EndOfWait` (delegate `Slot_Event`))
    (`self.Consume`)
    (`self.SetActorEnableCollision` _tool false)
    (set `self.Eating` true)
    (`KismetSystemLibrary.Delay` 4.0)
    (set `self.Eating` false)
    (`self.SetActorEnableCollision` _tool true)
    (`ActorComponent.Deactivate` (`self.NS_Eat`))
    (`self.Reward`)
    (`self.Leave`)))

(fn `ApplyName`
  (`self.SetActorHiddenInGame` (== (`self.Name`) 0))
  (`self.ChangedName`)
  (bind (_success _client) (`/Game/DataBase/Client/FL_Client.GetClient` (`self.Name`)))
  (if _success
    (`|ExecutionSequence`
      (:`then_0`
        (bind ((`SkeletalMesh_17_598B27AD496714080E6F0795A62C258E` _skeletalmesh) (`Animation_41_E318BC0A44FD95F1D30C39B7B6894458` _animation)) (break `/Game/DataBase/Client/ST_Client` _client))
        (bind _returnvalue (`KismetSystemLibrary.LoadAsset_Blocking` (select `bool` _success :`false` (`self.DefaultSkeletalMesh`) :`true` _skeletalmesh) :!label _label))
        (`SkeletalMeshComponent.SetSkeletalMeshAsset` (`self.Mesh`) (cast `SkeletalMesh` _returnvalue :!pure true)))
      (:`then_1`
        (bind _returnvalue_2 (`KismetSystemLibrary.LoadClassAsset_Blocking` _animation))
        (`SkeletalMeshComponent.SetAnimInstanceClass` (`self.Mesh`) _returnvalue_2)))
    (else
      (goto _label))))

(fn `ApplyPaused`
  (if (`self.Paused`)
    (`KismetSystemLibrary.K2_PauseTimerHandle` (`self.WaitTimer`))
    (else
      (`KismetSystemLibrary.K2_UnPauseTimerHandle` (`self.WaitTimer`)))))

(fn `ApplyStory`
  (if (!= (`self.Story`) 0)
    (`/Game/Blueprints/Systems/GSB_BearistaCoffee.AddProgression` (`/Game/Blueprints/Systems/FL_System.GetGSB_BearistaCoffee`) (`self.Story`))
    (`self.ChangedStory` (`self.Story`))))

(fn `Consume`
  (`|ExecutionSequence`
    (:`then_0`
      (bind _asbp_cup (cast `/Game/Blueprints/Actors/Tools/Instances/BP_Cup` (`/Game/Blueprints/Actors/Slots/AC_Slot.GetTool` (`self.GetComponentByClass` (`self.Spot`) "/Game/Blueprints/Actors/Slots/AC_Slot.AC_Slot_C") (`self.CupSlot`))))
      (`/Game/Blueprints/Actors/Tools/Instances/BP_Cup.Clear` _asbp_cup true))
    (:`then_1`
      (bind _asbp_pastrie (cast `/Game/Blueprints/Actors/Tools/Instances/BP_Pastrie` (`/Game/Blueprints/Actors/Slots/AC_Slot.GetTool` (`self.GetComponentByClass` (`self.Spot`) "/Game/Blueprints/Actors/Slots/AC_Slot.AC_Slot_C") (`self.PastrieSlot`))))
      (`/Game/Blueprints/Actors/Tools/BP_Tool.ToPool` _asbp_pastrie))
    (:`then_2`
      (`NiagaraComponent.ResetSystem` (`self.NS_Eat`))
      (`ActorComponent.Activate` (`self.NS_Eat`) false))))

(fn `CupMatchDrink`
  (returns (Match :type Boolean))
  (bind _asbp_cup (cast `/Game/Blueprints/Actors/Tools/Instances/BP_Cup` (`/Game/Blueprints/Actors/Slots/AC_Slot.GetTool` (`self.GetComponentByClass` (`self.Spot`) "/Game/Blueprints/Actors/Slots/AC_Slot.AC_Slot_C") (`self.CupSlot`)))
    (:`then`
      (bind (_success _drink) (`/Game/DataBase/Drink/FL_Drink.GetDrink` (`self.Drink`)))
      (if _success
        (return (`/Game/Blueprints/Actors/Tools/Instances/BP_Cup.IsDrink` _asbp_cup _drink))
        (else
          _)))
    (:`CastFailed`
      _))
  (return false))

(fn `EndOfWait`
  (params (SlotDelegate :type "Delegate (by ref)"))
  (bind _returnvalue (`self.GetComponentByClass` (`self.Spot`) "/Game/Blueprints/Actors/Slots/AC_Slot.AC_Slot_C"))
  (`KismetSystemLibrary.K2_ClearAndInvalidateTimerHandle` (`self.WaitTimer`))
  (remove `/Game/Blueprints/Actors/Slots/AC_Slot.Slotted` _returnvalue SlotDelegate)
  (remove `/Game/Blueprints/Actors/Slots/AC_Slot.Unslotted` _returnvalue SlotDelegate))

(fn `GetDrink`
  (returns (Drink :type "/Game/DataBase/Drink/EN_Drink Enum"))
  (return (`self.Drink`)))

(fn `GetName`
  (returns (Name :type "/Game/DataBase/Client/EN_Client Enum"))
  (return (`self.Name`)))

(fn `GetOrderDelay`
  (returns (OrderDelay :type "Float (double-precision)"))
  (bind ((`OrderDelay_15_8B885D8A4B34F7BEB1F48996BC146A05` _orderdelay) (`DoseDelay_12_72B15A2544B390688827558A41435B3E` _dosedelay) (`ExtraDelay_13_1743B8F041906EBFD25C5A977A53AAD7` _extradelay) (`PastrieDelay_14_79BF2915428C510FCC479BB6D3849436` _pastriedelay)) (break `/Game/DataBase/Difficulty/ST_Difficulty` (`/Game/Blueprints/Systems/GSB_BearistaCoffee.GetDifficultyData` (`/Game/Blueprints/Systems/FL_System.GetGSB_BearistaCoffee`))))
  (bind (_success _drink) (`/Game/DataBase/Drink/FL_Drink.GetDrink` (`self.Drink`)))
  (bind ((`Dose_5_72F6A0274AADC374312723B76F57A0FB` _dose) (`Extra1_10_A44E495D4EE54460F9E91E898EA38897` _extra1) (`Extra2_11_A1BC7A6045227DB12B37CEAC2341F112` _extra2)) (break `/Game/DataBase/Drink/ST_Drink` _drink))
  (return (+ (+ (+ (+ _orderdelay (`KismetMathLibrary.SelectFloat` _dosedelay 0.0 (!= _dose 0))) (`KismetMathLibrary.SelectFloat` _extradelay 0.0 (!= _extra1 0))) (`KismetMathLibrary.SelectFloat` _extradelay 0.0 (!= _extra2 0))) (`KismetMathLibrary.SelectFloat` _pastriedelay 0.0 (!= (`self.Pastrie`) 0)))))

(fn `GetOrderPawies`
  (returns (ReturnValue :type Integer))
  (bind (_success _drink) (`/Game/DataBase/Drink/FL_Drink.GetDrink` (`self.Drink`)))
  (bind (_success_2 _pastrie) (`/Game/DataBase/Pastrie/FL_Pastrie.GetPastrie` (`self.Pastrie`)))
  (return (+ (`.Pawies_8_B795D1D34271863273C325856DBA9327` (break `/Game/DataBase/Pastrie/ST_Pastrie` _pastrie)) (`.Pawies_18_6AF2EABE458552C6E9EC8CAC3F0A25BD` (break `/Game/DataBase/Drink/ST_Drink` _drink)))))

(fn `GetPastrie`
  (returns (Pastrie :type "/Game/DataBase/Pastrie/EN_Pastrie Enum"))
  (return (`self.Pastrie`)))

(fn `GetStory`
  (returns (Story :type "/Game/DataBase/Story/EN_Story Enum"))
  (return (`self.Story`)))

(fn `GetWait`
  (returns (WaitTimer :type "TimerHandle Structure"))
  (return (`self.WaitTimer`)))

(fn `GetWalk`
  (returns (WalkTimer :type "TimerHandle Structure"))
  (return (`self.WalkTimer`)))

(fn `PastrieMatchPastrie`
  (returns (Match :type Boolean))
  (locals (LocalPastrieSlotKey :type "/Game/Blueprints/Actors/Slots/ST_SlotKey Structure"))
  (if (!= (`self.Pastrie`) 0)
    (bind _asbp_pastrie (cast `/Game/Blueprints/Actors/Tools/Instances/BP_Pastrie` (`/Game/Blueprints/Actors/Slots/AC_Slot.GetTool` (`self.GetComponentByClass` (`self.Spot`) "/Game/Blueprints/Actors/Slots/AC_Slot.AC_Slot_C") (`self.PastrieSlot`)))
      (:`then`
        (return (`|EnumEquality` (`/Game/Blueprints/Actors/Tools/Instances/BP_Pastrie.GetPastrie` _asbp_pastrie) (`self.Pastrie`))))
      (:`CastFailed`
        (return false)))
    (else
      (return (not (`.Success` (`/Game/Blueprints/Actors/Slots/AC_Slot.GetTool` (`self.GetComponentByClass` (`self.Spot`) "/Game/Blueprints/Actors/Slots/AC_Slot.AC_Slot_C") (`self.PastrieSlot`))))))))

(fn `Punish`
  (locals (LocalGSB :type "/Game/Blueprints/Systems/GSB_BearistaCoffee Object Reference"))
  (set `local.LocalGSB` (`/Game/Blueprints/Systems/FL_System.GetGSB_BearistaCoffee`))
  (`|ExecutionSequence`
    (:`then_0`
      (`/Game/Blueprints/Systems/GSB_BearistaCoffee.AddPopularity` (`local.LocalGSB`) (`KismetMathLibrary.FTrunc` (* (`.PopularityRatio_5_11D34A0346A804E27A1DA096CDB62043` (break `/Game/DataBase/Service/ST_Service` (`/Game/Blueprints/Systems/GSB_BearistaCoffee.GetServiceData` (`local.LocalGSB`)))) (`self.GetOrderPawies`) -1.0))))
    (:`then_1`
      (`/Game/Blueprints/Systems/GSB_BearistaCoffee.ResetService` (`local.LocalGSB`)))
    (:`then_2`
      (`NiagaraComponent.ResetSystem` (`self.NS_Grumble`))
      (`ActorComponent.Activate` (`self.NS_Grumble`) false)
      (`self.Punished`))))

(fn `RandomOrder`
  (returns (Drink :type "/Game/DataBase/Drink/EN_Drink Enum") (Pastrie :type "/Game/DataBase/Pastrie/EN_Pastrie Enum"))
  (bind (_success _client) (`/Game/DataBase/Client/FL_Client.GetClient` (`self.Name`)))
  (bind ((`Drinks_8_D06DDD88475B4F7D831E75B568380552` _drinks) (`Pastries_13_65BFF4154AC2CB93A2C3DCA4E76E63C5` _pastries)) (break `/Game/DataBase/Client/ST_Client` _client))
  (return (`KismetArrayLibrary.Array_Random` _drinks) (`KismetArrayLibrary.Array_Random` _pastries)))

(fn `Reward`
  (locals (LocalGSB :type "/Game/Blueprints/Systems/GSB_BearistaCoffee Object Reference"))
  (set `local.LocalGSB` (`/Game/Blueprints/Systems/FL_System.GetGSB_BearistaCoffee`))
  (`|ExecutionSequence`
    (:`then_0`
      (bind (_success _service) (`/Game/DataBase/Service/FL_Service.GetService` (`/Game/Blueprints/Systems/GSB_BearistaCoffee.GetServiceValue` (`local.LocalGSB`))))
      (`/Game/Blueprints/Systems/GSB_BearistaCoffee.AddPopularity` (`local.LocalGSB`) (`KismetMathLibrary.FTrunc` (* (`self.GetOrderPawies`) (`.PopularityRatio_5_11D34A0346A804E27A1DA096CDB62043` (break `/Game/DataBase/Service/ST_Service` _service))))))
    (:`then_1`
      (bind (_success_2 _popularity) (`/Game/DataBase/Popularity/FL_Popularity.GetPopularity` (`/Game/Blueprints/Systems/GSB_BearistaCoffee.GetPopularityValue` (`local.LocalGSB`))))
      (`/Game/Blueprints/Systems/GSB_BearistaCoffee.AddPawies` (`local.LocalGSB`) (`KismetMathLibrary.FTrunc` (* (`.PawiesRatio_9_4F3EA9F84C8CF94A04540BBAF7104760` (break `/Game/DataBase/Popularity/ST_Popularity` _popularity)) (`self.GetOrderPawies`)))))
    (:`then_2`
      (`/Game/Blueprints/Systems/GSB_BearistaCoffee.AddAffinity` (`local.LocalGSB`) (`self.Name`) (`self.GetOrderPawies`))
      (`self.SetStory` (`self.SelectStory`))
      (`/Game/Blueprints/Systems/GSB_BearistaCoffee.AddService` (`local.LocalGSB`) 1))
    (:`then_3`
      (`NiagaraComponent.ResetSystem` (`self.NS_Pay`))
      (`ActorComponent.Activate` (`self.NS_Pay`) false)
      (`self.Rewarded`))))

(fn `SelectStory`
  (returns (Story :type "/Game/DataBase/Story/EN_Story Enum"))
  (locals (LocalGSB :type "/Game/Blueprints/Systems/GSB_BearistaCoffee Object Reference"))
  (set `local.LocalGSB` (`/Game/Blueprints/Systems/FL_System.GetGSB_BearistaCoffee`))
  (bind (_success _client) (`/Game/DataBase/Client/FL_Client.GetClient` (`self.Name`)))
  (for _array_element (`.Stories_29_17E8B65D4BCDF233AC607480580F9F01` (break `/Game/DataBase/Client/ST_Client` _client))
    (bind (_success_2 _story) (`/Game/DataBase/Story/FL_Story.GetStory` _array_element))
    (bind ((`Affinity_6_A4CF009448ED631EB17D9AA7C6763D0C` _affinity) (`Requirements_16_4DF8BDDF407BA848C65B0E97DB43F9EC` _requirements)) (break `/Game/DataBase/Story/ST_Story` _story))
    (bind __ (`/Game/Blueprints/ML_Object.Contains` _requirements (`/Game/Blueprints/Systems/GSB_BearistaCoffee.GetProgression` (`local.LocalGSB`))))
    (if (and __ (< _affinity (`/Game/Blueprints/Systems/GSB_BearistaCoffee.GetAffinity` (`local.LocalGSB`) (`self.Name`))) (not (`KismetArrayLibrary.Array_Contains` (`/Game/Blueprints/Systems/GSB_BearistaCoffee.GetProgression` (`local.LocalGSB`)) _array_element)))
      (return _array_element)))
  (return "NewEnumerator0"))

(fn `ServiceMatchOrder`
  (returns (Match :type Boolean))
  (locals (LocalCupSlotKey :type "/Game/Blueprints/Actors/Slots/ST_SlotKey Structure" :default (struct :`ToolClass` "/Game/Blueprints/Actors/Tools/Instances/BP_Cup.BP_Cup_C" :`RelativeTransform` (struct :`Rotation` (struct :`W` 1.0) :`Translation` (0.0 0.0 0.0) :`Scale3D` (1.0 1.0 1.0)))) (LocalPastrieSlotKey :type "/Game/Blueprints/Actors/Slots/ST_SlotKey Structure" :default (struct :`ToolClass` "/Game/Blueprints/Actors/Tools/Instances/BP_Pastrie.BP_Pastrie_C" :`RelativeTransform` (struct :`Rotation` (struct :`W` 1.0) :`Translation` (0.0 0.0 0.0) :`Scale3D` (1.0 1.0 1.0)))))
  (return (and (`self.CupMatchDrink`) (`self.PastrieMatchPastrie`))))

(fn `SetName`
  (params (Name :type "/Game/DataBase/Client/EN_Client Enum" :default "NewEnumerator0"))
  (set `self.Name` Name)
  (`self.ApplyName`))

(fn `SetOrder`
  (params (Drink :type "/Game/DataBase/Drink/EN_Drink Enum" :default "NewEnumerator0") (Pastrie :type "/Game/DataBase/Pastrie/EN_Pastrie Enum" :default "NewEnumerator0"))
  (set `self.Drink` Drink)
  (set `self.Pastrie` Pastrie)
  (`self.ChangedOrder`))

(fn `SetPaused`
  (params (Paused :type Boolean))
  (set `self.Paused` Paused)
  (`self.ApplyPaused`))

(fn `SetStory`
  (params (Story :type "/Game/DataBase/Story/EN_Story Enum" :default "NewEnumerator0"))
  (set `self.Story` Story)
  (`self.ApplyStory`))

(fn `UserConstructionScript`
  (`self.ApplyName`))