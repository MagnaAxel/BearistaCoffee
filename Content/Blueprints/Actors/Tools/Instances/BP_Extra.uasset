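; BP_Extra is a tool actor whose static mesh shows the Extra assigned to it.
; ApplyExtra looks up that Extra's data and sets its mesh, falling back to a default mesh when the lookup fails.
; The construction script and SetExtra both run ApplyExtra, and SetExtra also reports the change through debug feedback.
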(fn `ApplyExtra`
  (bind (_success _extra) (`/Game/DataBase/Extra/FL_Extra.GetExtra` (`self.Extra`)))
  (`StaticMeshComponent.SetStaticMesh` (`self.StaticMesh`) (`|ConvertAsset` (select `bool` _success :`false` (`self.DefaultStaticMesh`) :`true` (`.StaticMesh_6_611483ED41166C50C19A7B8D6F2F1E13` (break `/Game/DataBase/Extra/ST_Extra` _extra))))))

(fn `GetExtra`
  (returns (Extra :type "/Game/DataBase/Extra/EN_Extra Enum"))
  (return (`self.Extra`)))

(fn `SetExtra`
  (params (Extra :type "/Game/DataBase/Extra/EN_Extra Enum" :default "NewEnumerator0"))
  ; Action
  (set `self.Extra` Extra)
  ; FeedBack
  (`self.ApplyExtra`)
  (`/Game/Blueprints/FL_Common.DebugFeedBack` self "SetExtra" true))

(fn `UserConstructionScript`
  (`self.ApplyExtra`))