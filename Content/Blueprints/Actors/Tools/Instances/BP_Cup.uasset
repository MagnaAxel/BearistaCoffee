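; BP_Cup is a tool actor for a drink cup that holds one dose, up to two extras and a filthy flag.
; Content changes and construction call ApplyDrink, which looks up the matching drink and sets its mesh, falling back to a default.
; An extra added to a full cup marks it filthy, while a rejected dose clears the flag.
; ApplyFilthy is an empty feedback hook, and actions report through DebugFeedBack.
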(fn `AddDose`
  (params (Dose :type "/Game/DataBase/Dose/EN_Dose Enum" :default "NewEnumerator0"))
  (returns (Success :type Boolean))
  ; Condition
  (if (== (`self.Dose`) 0)
    ; Action
    (set `self.Dose` Dose)
    ; FeedBack
    (`self.ApplyDrink`)
    (`/Game/Blueprints/FL_Common.DebugFeedBack` self "AddDose" true)
    (return true)
    (else
      (`self.SetFilthy` false)
      (`/Game/Blueprints/FL_Common.DebugFeedBack` self "AddDose")
      (return false))))

(fn `AddExtra`
  (params (Extra :type "/Game/DataBase/Extra/EN_Extra Enum" :default "NewEnumerator0"))
  (returns (Success :type Boolean))
  (`|ExecutionSequence`
    (:`then_0`
      ; Condition
      (if (== (`self.Extra1`) 0)
        ; Action
        (set `self.Extra1` Extra)
        ; FeedBack
        (`self.ApplyDrink`)
        (`/Game/Blueprints/FL_Common.DebugFeedBack` self "AddExtra" true)
        (return true)))
    (:`then_1`
      (if (== (`self.Extra2`) 0)
        (set `self.Extra2` Extra)
        (`self.ApplyDrink`)
        (`/Game/Blueprints/FL_Common.DebugFeedBack` self "AddExtra" true)
        (return true)))
    (:`then_2`
      (`self.SetFilthy` true)
      (`/Game/Blueprints/FL_Common.DebugFeedBack` self "AddExtra")
      (return false))))

(fn `ApplyDrink`
  (bind (_success _drink) (`/Game/DataBase/Drink/FL_Drink.GetDrinkByCup` self))
  (`StaticMeshComponent.SetStaticMesh` (`self.StaticMesh`) (`|ConvertAsset` (select `bool` _success :`false` (`self.DefaultStaticMesh`) :`true` (`.StaticMesh_14_F402B1DC435053A0D483CEB764FC4612` (break `/Game/DataBase/Drink/ST_Drink` _drink))))))

(fn `ApplyFilthy`)

(fn `Clear`
  (params (Filthy :type Boolean))
  ; Action
  (`self.SetFilthy` Filthy)
  (set `self.Dose` "NewEnumerator0")
  (set `self.Extra1` "NewEnumerator0")
  (set `self.Extra2` "NewEnumerator0")
  ; DebugFeedback
  (`self.ApplyDrink`)
  (`/Game/Blueprints/FL_Common.DebugFeedBack` self "Clear" true))

(fn `IsClear`
  (returns (Clear :type Boolean))
  (return (and (`self.IsEmpty`) (not (`self.IsFilthy`)))))

(fn `IsDrink`
  (params (Drink :type "/Game/DataBase/Drink/ST_Drink Structure"))
  (returns (Match :type Boolean))
  (bind ((`Dose_5_72F6A0274AADC374312723B76F57A0FB` _dose) (`Extra1_10_A44E495D4EE54460F9E91E898EA38897` _extra1) (`Extra2_11_A1BC7A6045227DB12B37CEAC2341F112` _extra2)) (break `/Game/DataBase/Drink/ST_Drink` Drink))
  (bind _array (`|MakeArray` (`self.Extra1`) (`self.Extra2`)))
  (return (and (== _dose 0) (`KismetArrayLibrary.Array_Contains` _array _extra1) (`KismetArrayLibrary.Array_Contains` _array _extra2))))

(fn `IsEmpty`
  (returns (Empty :type Boolean))
  (return (and (== (`self.Dose`) 0) (== (`self.Extra1`) 0) (== (`self.Extra2`) 0))))

(fn `IsFilthy`
  (returns (Filthy :type Boolean))
  (return (`self.Filthy`)))

(fn `SetFilthy`
  (params (Filthy :type Boolean))
  ; Action
  (set `self.Filthy` Filthy)
  ; FeedBack
  (`self.ApplyFilthy`)
  (`/Game/Blueprints/FL_Common.DebugFeedBack` self "SetFilthy"))

(fn `UserConstructionScript`
  (`self.ApplyDrink`))