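; BP_Pastrie is a tool actor that displays a pastry, with its static mesh chosen by the Pastrie variable.
; ApplyPastrie runs at construction and after SetPastrie, looking up the pastry's data and falling back to a default mesh if the lookup fails.
; The soft mesh reference is loaded synchronously before being applied to the StaticMesh component.
; SetPastrie also logs debug feedback, and GetPastrie exposes the current value.
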(fn `ApplyPastrie`
  (bind (_success _pastrie) (`/Game/DataBase/Pastrie/FL_Pastrie.GetPastrie` (`self.Pastrie`)))
  (bind _returnvalue (`KismetSystemLibrary.LoadAsset_Blocking` (select `bool` _success :`false` (`self.DefaultStaticMesh`) :`true` (`.StaticMesh_5_11D0790F46958EEEDE4299A0008DDB5A` (break `/Game/DataBase/Pastrie/ST_Pastrie` _pastrie)))))
  (bind _asstatic_mesh (cast `StaticMesh` _returnvalue))
  (`StaticMeshComponent.SetStaticMesh` (`self.StaticMesh`) _asstatic_mesh))

(fn `GetPastrie`
  (returns (Pastrie :type "/Game/DataBase/Pastrie/EN_Pastrie Enum"))
  (return (`self.Pastrie`)))

(fn `SetPastrie`
  (params (Pastrie :type "/Game/DataBase/Pastrie/EN_Pastrie Enum" :default "NewEnumerator0"))
  ; Action
  (set `self.Pastrie` Pastrie)
  ; FeedBack
  (`self.ApplyPastrie`)
  (`/Game/Blueprints/FL_Common.DebugFeedBack` self "SetPastrie" true))

(fn `UserConstructionScript`
  (`self.ApplyPastrie`))