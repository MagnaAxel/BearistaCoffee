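; Base logic for a tool actor that can be caught by an actor, released into a slot on a static, or sent back to its pool.
; Catch unslots the tool from its attach parent, then attaches it to the catcher, with a timeline lerping it toward a relative transform on that moving target.
; Release finds a static within trace range and tries to slot into it, while ToPool slots the tool into its pool.
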(event `Attach`
  (params (Actor :type "Actor Object Reference (by ref)") (RelativeTransform :type "Transform Structure"))
  ; Action
  (`self.K2_AttachToActor` Actor "None" "KeepWorld" "KeepWorld" "KeepWorld" false)
  (set `self.StartTransform` (`self.GetTransform` self))
  (bind (_direction _alpha) (`Timeline|MoveToActorTimeline` :!via `PlayFromStart`)
    (:`Update`
      (`self.K2_SetActorTransform` (`KismetMathLibrary.TLerp` (`self.StartTransform`) (`KismetMathLibrary.ComposeTransforms` RelativeTransform (`self.GetTransform` Actor)) _alpha)))
    (:`Finished`
      ; FeedBack
      (`/Game/Blueprints/FL_Common.DebugFeedBack` self "Attach" true))))

(fn `Catch`
  (params (Actor :type "Actor Object Reference") (RelativeTransform :type "Transform Structure"))
  (returns (Success :type Boolean))
  (bind _success (`/Game/Blueprints/Actors/Slots/FL_Slot.TryUnslot` (`self.GetAttachParentActor`) Actor self))
  (if _success
    (`self.Attach` Actor RelativeTransform)
    (`self.Catched`)
    (return true)))

(fn `Release`
  (params (Actor :type "Actor Object Reference"))
  (returns (Success :type Boolean))
  (bind (_success _static) (`/Game/Blueprints/FL_Common.FindStatic` self (`self.LineTraceRange`)))
  (bind _success_2 (`/Game/Blueprints/Actors/Slots/FL_Slot.TrySlot` _static Actor self))
  (if _success_2
    (`self.Released`)
    (return true)
    (else
      (return false))))

(fn `ToPool`
  ; Action
  (bind _success (`/Game/Blueprints/Actors/Slots/FL_Slot.TrySlot` (`self.Pool`) self self))
  ; FeedBack
  (`/Game/Blueprints/FL_Common.DebugFeedBack` self "ToPool" _success))

(fn `UserConstructionScript`
  (`StaticMeshComponent.SetStaticMesh` (`self.StaticMesh`) (`|ConvertAsset` (`self.DefaultStaticMesh`))))