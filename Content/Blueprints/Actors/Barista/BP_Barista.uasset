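; Player barista character with camera-relative movement, two-handed tool catch and release via ACHandSlot, and interaction and navigation on traced statics.
; An overlap sphere sized from trace range shows widget prompts and snaps facing to the nearest actor before hand actions.
; Run presses stack speed that a timeline decays, scaling trail particles; hits at speed bounce the character with stun VFX.
; A lock counter gates input actions.
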(event `self.ReceiveBeginPlay`
  (set `CharacterMovementComponent.MaxWalkSpeed` (`self.BaseWalkSpeed`) (`self.CharacterMovement`))
  (bind _returnvalue (`GameplayStatics.GetActorOfClass` "/Script/Engine.CameraActor"))
  (set `self.Camera` _returnvalue))

(event `self.CapsuleComponent.OnComponentHit`
  (params (HitComponent :type "PrimitiveComponent Object Reference") (OtherActor :type "Actor Object Reference") (OtherComp :type "PrimitiveComponent Object Reference") (NormalImpulse :type "Vector Structure") (Hit :type "HitResult Structure (by ref)"))
  (bind _ns_stun (`self.NS_Stun`))
  (if (> (`CharacterMovementComponent.MaxWalkSpeed` (`self.CharacterMovement`)) (`self.BumpWalkSpeed`))
    (`self.LaunchCharacter` (* (`KismetMathLibrary.MakeVector` (.x (`KismetMathLibrary.MirrorVectorByNormal` (`self.GetActorForwardVector` self) (`.Normal` (`GameplayStatics.BreakHitResult` Hit)))) (.y (`KismetMathLibrary.MirrorVectorByNormal` (`self.GetActorForwardVector` self) (`.Normal` (`GameplayStatics.BreakHitResult` Hit))))) (`CharacterMovementComponent.MaxWalkSpeed` (`self.CharacterMovement`))) true)
    (`TimelineComponent.Stop` (`self.DecreaseWalkSpeedTimeline`))
    (set `CharacterMovementComponent.MaxWalkSpeed` (`self.BaseWalkSpeed`) (`self.CharacterMovement`))
    (`NiagaraComponent.ResetSystem` _ns_stun)
    (`ActorComponent.Activate` _ns_stun false)))

(event `/Game/Blueprints/Actors/Barista/IN_Lock.Lock`
  (`/Engine/EditorBlueprintResources/StandardMacros.IncrementInt` (`self.LockCount`)
    (:`  `
      (`/Game/Blueprints/FL_Common.DebugFeedBack` self "Lock" true))))

(event `/Game/Blueprints/Actors/Barista/IN_Lock.UnLock`
  (set `self.LockCount` (`KismetMathLibrary.Max` (- (`self.LockCount`) 1)))
  (`/Game/Blueprints/FL_Common.DebugFeedBack` self "Unlock" true))

(event `EnhancedInput|/Game/Blueprints/Systems/Controller/InputActions/IA_Move`
  (params (ActionValue :type "Vector2D Structure") (ElapsedSeconds :type "Float (double-precision)") (TriggeredSeconds :type "Float (double-precision)") (InputAction :type "InputAction Object Reference" :default "/Game/Blueprints/Systems/Controller/InputActions/IA_Move.IA_Move"))
  (bind (_returnvalue_roll _returnvalue_pitch _returnvalue_yaw) (`KismetMathLibrary.BreakRotator` (`SceneComponent.K2_GetComponentRotation` (`Actor.RootComponent` (`self.Camera`)))))
  (:`Triggered`
    (`self.IsLockedBranch`
      (:`False`
        (`self.AddMovementInput` (`KismetMathLibrary.GreaterGreater_VectorRotator` (`KismetMathLibrary.Conv_Vector2DToVector` ActionValue) (`KismetMathLibrary.MakeRotator` 0.0 0.0 _returnvalue_yaw))))))
  (:`Started`
    (`NiagaraComponent.ResetSystem` (`self.NS_Displacement`))
    (`ActorComponent.Activate` (`self.NS_Displacement`) false))
  (:`Completed`
    (`ActorComponent.Deactivate` (`self.NS_Displacement`))))

(event `EnhancedInput|/Game/Blueprints/Systems/Controller/InputActions/IA_Run`
  (params (ActionValue :type Boolean) (ElapsedSeconds :type "Float (double-precision)") (TriggeredSeconds :type "Float (double-precision)") (InputAction :type "InputAction Object Reference" :default "/Game/Blueprints/Systems/Controller/InputActions/IA_Run.IA_Run"))
  (bind _ns_displacement (`self.NS_Displacement`))
  (bind _ns_displacement_2 (`self.NS_Displacement`))
  (:`Triggered`
    (`self.IsLockedBranch`
      (:`False`
        (if (!= (`|GetInputActionValue`) (0.0 0.0))
          (bind _output_get (set `CharacterMovementComponent.MaxWalkSpeed` (`KismetMathLibrary.FMin` (+ (`CharacterMovementComponent.MaxWalkSpeed` (`self.CharacterMovement`)) (`self.AdditiveWalkSpeed`)) (`self.LimitWalkSpeed`)) (`self.CharacterMovement`)))
          (set `self.TopWalkSpeed` _output_get)
          (`|ExecutionSequence`
            (:`then_0`
              (bind (_direction _alpha) (`Timeline|DecreaseWalkSpeedTimeline` :!via `PlayFromStart`)
                (:`Update`
                  (bind _output_get_2 (set `CharacterMovementComponent.MaxWalkSpeed` (`KismetMathLibrary.Lerp` (`self.TopWalkSpeed`) (`self.BaseWalkSpeed`) _alpha) (`self.CharacterMovement`)))
                  (`|ExecutionSequence`
                    (:`then_0`
                      (bind _returnvalue (`KismetMathLibrary.Lerp` 0.5 1.0 (/ _output_get_2 (`self.TopWalkSpeed`))))
                      (`FXSystemComponent.SetFloatParameter` _ns_displacement_2 "Lifetime_Min" (- _returnvalue 0.5))
                      (`FXSystemComponent.SetFloatParameter` _ns_displacement_2 "Lifetime_Max" _returnvalue))
                    (:`then_1`
                      (`FXSystemComponent.SetFloatParameter` _ns_displacement "Mesh_Size_Min" _returnvalue)
                      (`FXSystemComponent.SetFloatParameter` _ns_displacement "Mesh_Size_Max" (+ _returnvalue 0.5)))))
                (:`Finished`)))
            (:`then_1`
              (`/Game/Blueprints/FL_Common.DebugFeedBack` self "Run" true))))))))

(event `EnhancedInput|/Game/Blueprints/Systems/Controller/InputActions/IA_Interact`
  (params (ActionValue :type Boolean) (ElapsedSeconds :type "Float (double-precision)") (TriggeredSeconds :type "Float (double-precision)") (InputAction :type "InputAction Object Reference" :default "/Game/Blueprints/Systems/Controller/InputActions/IA_Interact.IA_Interact"))
  (:`Triggered`
    (`self.IsLockedBranch`
      (:`False`
        (bind (_success _static) (`/Game/Blueprints/FL_Common.FindStatic` self (`self.LineTraceRange`)))
        (bind _success_2 (`/Game/Blueprints/Actors/Interactives/FL_Interactive.TryInteract` _static))
        (`/Game/Blueprints/FL_Common.DebugFeedBack` self "Interact" _success_2)))))

(event `EnhancedInput|/Game/Blueprints/Systems/Controller/InputActions/IA_Navigate`
  (params (ActionValue :type "Vector2D Structure") (ElapsedSeconds :type "Float (double-precision)") (TriggeredSeconds :type "Float (double-precision)") (InputAction :type "InputAction Object Reference" :default "/Game/Blueprints/Systems/Controller/InputActions/IA_Navigate.IA_Navigate"))
  (bind (_x _y) (`KismetMathLibrary.BreakVector2D` ActionValue))
  (:`Triggered`
    (`self.IsLockedBranch`
      (:`False`
        (bind (_success _static) (`/Game/Blueprints/FL_Common.FindStatic` self (`self.LineTraceRange`)))
        (`|ExecutionSequence`
          (:`then_0`
            (if (> _x 0.9)
              (bind _success_2 (`/Game/Blueprints/Actors/Slots/Navigations/FL_Navigation.TryRight` _static))
              (`/Game/Blueprints/FL_Common.DebugFeedBack` self "Navigation Right" _success_2)))
          (:`then_1`
            (if (< _x -0.9)
              (bind _success_3 (`/Game/Blueprints/Actors/Slots/Navigations/FL_Navigation.TryLeft` _static))
              (`/Game/Blueprints/FL_Common.DebugFeedBack` self "Navigation Left" _success_3)))
          (:`then_2`
            (if (> _y 0.9)
              (bind _success_4 (`/Game/Blueprints/Actors/Slots/Navigations/FL_Navigation.TryDown` _static))
              (`/Game/Blueprints/FL_Common.DebugFeedBack` self "Navigation Down" _success_4)))
          (:`then_3`
            (if (< _y -0.9)
              (bind _success_5 (`/Game/Blueprints/Actors/Slots/Navigations/FL_Navigation.TryUp` _static))
              (`/Game/Blueprints/FL_Common.DebugFeedBack` self "Navigation Up" _success_5))))))))

(event `EnhancedInput|/Game/Blueprints/Systems/Controller/InputActions/IA_HandRight`
  (params (ActionValue :type Boolean) (ElapsedSeconds :type "Float (double-precision)") (TriggeredSeconds :type "Float (double-precision)") (InputAction :type "InputAction Object Reference" :default "/Game/Blueprints/Systems/Controller/InputActions/IA_HandRight.IA_HandRight"))
  (bind _value (`self.GetHandRight`))
  (:`Triggered`
    (`self.IsLockedBranch`
      (:`False`
        (`self.AimAssist`)
        (if (`KismetSystemLibrary.IsValid` _value)
          (bind _success (`/Game/Blueprints/Actors/Tools/FL_Tool.TryRelease` _value self))
          (`/Game/Blueprints/FL_Common.DebugFeedBack` self "Release Right" _success)
          (else
            (bind (_success_2 _tool) (`/Game/Blueprints/FL_Common.FindTool` self (`self.LineTraceRange`) (`|MakeArray` (`BlueprintMapLibrary.Map_Find` (`/Game/Blueprints/Actors/Slots/AC_Slot.Tools` (`self.AC_HandSlot`)) (`self.HandRightSlotKey`)) (`BlueprintMapLibrary.Map_Find` (`/Game/Blueprints/Actors/Slots/AC_Slot.Tools` (`self.AC_HandSlot`)) (`self.HandLeftSlotKey`)))))
            (if _success_2
              (bind _success_3 (message `/Game/Blueprints/Actors/Slots/IN_Slot.SlotAt` (`self.AC_HandSlot`) self _tool (`self.HandRightSlotKey`)))
              (`/Game/Blueprints/FL_Common.DebugFeedBack` self "Catch Right" _success_3))))))))

(event `EnhancedInput|/Game/Blueprints/Systems/Controller/InputActions/IA_HandLeft`
  (params (ActionValue :type Boolean) (ElapsedSeconds :type "Float (double-precision)") (TriggeredSeconds :type "Float (double-precision)") (InputAction :type "InputAction Object Reference" :default "/Game/Blueprints/Systems/Controller/InputActions/IA_HandLeft.IA_HandLeft"))
  (bind _value (`self.GetHandLeft`))
  (:`Triggered`
    (`self.IsLockedBranch`
      (:`False`
        (`self.AimAssist`)
        (if (`KismetSystemLibrary.IsValid` _value)
          (bind _success (`/Game/Blueprints/Actors/Tools/FL_Tool.TryRelease` _value self))
          (`/Game/Blueprints/FL_Common.DebugFeedBack` self "Release left" _success)
          (else
            (bind (_success_2 _tool) (`/Game/Blueprints/FL_Common.FindTool` self (`self.LineTraceRange`) (`|MakeArray` (`BlueprintMapLibrary.Map_Find` (`/Game/Blueprints/Actors/Slots/AC_Slot.Tools` (`self.AC_HandSlot`)) (`self.HandRightSlotKey`)) (`BlueprintMapLibrary.Map_Find` (`/Game/Blueprints/Actors/Slots/AC_Slot.Tools` (`self.AC_HandSlot`)) (`self.HandLeftSlotKey`)))))
            (if _success_2
              (bind _success_3 (message `/Game/Blueprints/Actors/Slots/IN_Slot.SlotAt` (`self.AC_HandSlot`) self _tool (`self.HandLeftSlotKey`)))
              (`/Game/Blueprints/FL_Common.DebugFeedBack` self "Catch left" _success_3))))))))

(event `self.AimAssistCollision.OnComponentBeginOverlap`
  (params (OverlappedComponent :type "PrimitiveComponent Object Reference") (OtherActor :type "Actor Object Reference") (OtherComp :type "PrimitiveComponent Object Reference") (OtherBodyIndex :type Integer) (bFromSweep :type Boolean) (SweepResult :type "HitResult Structure (by ref)"))
  (`KismetArrayLibrary.Array_AddUnique` (`self.AimAssistPool`) OtherActor)
  (bind _returnvalue (`self.GetComponentByClass` OtherActor "/Script/UMG.WidgetComponent"))
  (`/Engine/EditorBlueprintResources/StandardMacros.IsValid` _returnvalue
    (:`Is Valid`
      (message `/Game/Blueprints/Widgets/Interfaces/IN_HideWidget.ShowWidget` (`WidgetComponent.GetWidget` _returnvalue)))))

(event `self.AimAssistCollision.OnComponentEndOverlap`
  (params (OverlappedComponent :type "PrimitiveComponent Object Reference") (OtherActor :type "Actor Object Reference") (OtherComp :type "PrimitiveComponent Object Reference") (OtherBodyIndex :type Integer))
  (`KismetArrayLibrary.Array_RemoveItem` (`self.AimAssistPool`) OtherActor)
  (bind _returnvalue (`self.GetComponentByClass` OtherActor "/Script/UMG.WidgetComponent"))
  (`/Engine/EditorBlueprintResources/StandardMacros.IsValid` _returnvalue
    (:`Is Valid`
      (message `/Game/Blueprints/Widgets/Interfaces/IN_HideWidget.HideWidget` (`WidgetComponent.GetWidget` _returnvalue)))))

(event `AimAssist`
  (bind (_distance _returnvalue) (`GameplayStatics.FindNearestActor` (`self.K2_GetActorLocation` self) (`self.AimAssistPool`)))
  (if (< _distance (`self.LineTraceRange`))
    (`self.K2_SetActorRotation` self (`KismetMathLibrary.FindLookAtRotation` (`self.K2_GetActorLocation` self) (`self.K2_GetActorLocation` _returnvalue)) false)))

(fn `GetHandLeft`
  (returns (Value :type "Actor Object Reference"))
  (bind _ac_handslot (`self.AC_HandSlot`))
  (`/Engine/EditorBlueprintResources/StandardMacros.IsValid` _ac_handslot
    (:`Is Valid`
      (return (`BlueprintMapLibrary.Map_Find` (`/Game/Blueprints/Actors/Slots/AC_Slot.Tools` _ac_handslot) (`self.HandLeftSlotKey`))))
    (:`Is Not Valid`
      (return null))))

(fn `GetHandRight`
  (returns (Value :type "Actor Object Reference"))
  (bind _ac_handslot (`self.AC_HandSlot`))
  (`/Engine/EditorBlueprintResources/StandardMacros.IsValid` _ac_handslot
    (:`Is Valid`
      (return (`BlueprintMapLibrary.Map_Find` (`/Game/Blueprints/Actors/Slots/AC_Slot.Tools` _ac_handslot) (`self.HandRightSlotKey`))))
    (:`Is Not Valid`
      (return null))))

(fn `IsLocked`
  (returns (Locked :type Boolean))
  (return (> (`self.LockCount`) 0)))

(fn `SetAimAssistCollision`
  (locals (AimAssistSize :type "Float (double-precision)" :default 0.0))
  (set `local.AimAssistSize` (`KismetMathLibrary.Conv_IntToDouble` (/ (`self.LineTraceRange`) 2)))
  (`SceneComponent.K2_SetRelativeLocation` (`self.AimAssistCollision`) (`KismetMathLibrary.MakeVector` (- (`local.AimAssistSize`) (/ (`CapsuleComponent.CapsuleRadius` (`self.CapsuleComponent`)) 2.0))) false false)
  (`SphereComponent.SetSphereRadius` (`self.AimAssistCollision`) (+ (`local.AimAssistSize`) (/ (`CapsuleComponent.CapsuleRadius` (`self.CapsuleComponent`)) 2.0)) true))

(fn `UserConstructionScript`
  (`self.SetAimAssistCollision`))