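; AC_Action is a base actor component that runs a delayed action on its owner when the required tools are slotted.
; It listens to the owner's AC_Slot, starting a timer once all SlotKeys are valid and aborting it if unslotting breaks that.
; The timer fires the empty ActionFunction, a hook for subclasses.
; Shared macros handle optional locking of the slotted actor, tag-found Niagara feedback and Acting, Acted and Aborted dispatchers.
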(event `self.ReceiveBeginPlay`
  (bind _output_get (set `self.Slot` (`Actor.GetComponentByClass` (`self.GetOwner`) "/Game/Blueprints/Actors/Slots/AC_Slot.AC_Slot_C")))
  (add `/Game/Blueprints/Actors/Slots/AC_Slot.Slotted` _output_get (delegate `Slotted_Event`))
  (add `/Game/Blueprints/Actors/Slots/AC_Slot.Unslotted` _output_get (delegate `Unslotted_Event`)))

(event `Slotted_Event`
  (params (Actor :type "Actor Object Reference"))
  (set `self.Actor` Actor)
  (`self.Start`))

(event `Unslotted_Event`
  (params (Actor :type "Actor Object Reference"))
  (`self.Abort`))

(event `Action`
  (bind _returnvalue (`KismetSystemLibrary.K2_SetTimerDelegate` (delegate `Action_Event`) (`self.ActionDelay`)))
  (set `self.ActionTimer` _returnvalue)
  (if (`self.LockingAction`)
    (`/Game/Blueprints/Actors/Barista/FL_Lock.TryLock` (`self.Actor`)))
  (`self.Activate` (`Actor.FindComponentByTag` (`self.GetOwner`) "/Script/Niagara.NiagaraComponent" (`self.ActingTag`)) false)
  (`self.Acting`))

(event `Action_Event`
  (bind _returnvalue (`Actor.FindComponentByTag` (`self.GetOwner`) "/Script/Niagara.NiagaraComponent" (`self.ActedTag`)))
  (`KismetSystemLibrary.K2_ClearAndInvalidateTimerHandle` (`self.ActionTimer`))
  (`self.Action_Function`)
  (if (`self.LockingAction`)
    (`/Game/Blueprints/Actors/Barista/FL_Lock.TryUnlock` (`self.Actor`)))
  (`self.Deactivate` (`Actor.FindComponentByTag` (`self.GetOwner`) "/Script/Niagara.NiagaraComponent" (`self.ActingTag`)))
  (`NiagaraComponent.ResetSystem` _returnvalue)
  (`self.Activate` _returnvalue false)
  (`self.Acted`))

(fn `Abort`
  (returns (Success :type Boolean))
  ; Condition
  (if (`self.CanAbort`)
    ; Action
    (`KismetSystemLibrary.K2_ClearAndInvalidateTimerHandle` (`self.ActionTimer`))
    (if (`self.LockingAction`)
      (`/Game/Blueprints/Actors/Barista/FL_Lock.TryUnlock` (`self.Actor`)))
    ; FeedBack
    (`self.Deactivate` (`Actor.FindComponentByTag` (`self.GetOwner`) "/Script/Niagara.NiagaraComponent" (`self.ActingTag`)))
    (`self.Aborted`)
    (return true)
    (else
      (return false))))

(fn `Action_Function`)

(fn `CanAbort`
  (returns (Abort :type Boolean))
  (return (and (`KismetSystemLibrary.K2_IsValidTimerHandle` (`self.ActionTimer`)) (not (`self.CanAct`)))))

(fn `CanAct`
  (returns (Act :type Boolean))
  (for _array_element (`self.SlotKeys`)
    (if (not (`KismetSystemLibrary.IsValid` (`BlueprintMapLibrary.Map_Find` (`/Game/Blueprints/Actors/Slots/AC_Slot.Tools` (`self.Slot`)) _array_element)))
      (return false)))
  (return true))

(fn `CanStart`
  (returns (Start :type Boolean))
  (return (and (not (`KismetSystemLibrary.K2_IsValidTimerHandle` (`self.ActionTimer`))) (`self.CanAct`))))

(fn `GetTool`
  (params (Index :type Integer))
  (returns (Tool :type "Actor Object Reference"))
  (return (`/Game/Blueprints/Actors/Slots/AC_Slot.GetTool` (`self.Slot`) (`|GetArrayItem` (`self.SlotKeys`) Index))))

(fn `Start`
  (returns (Success :type Boolean))
  ; Condition
  (if (`self.CanStart`)
    ; Action
    (`self.Action`)
    (return true)
    (else
      (return false))))