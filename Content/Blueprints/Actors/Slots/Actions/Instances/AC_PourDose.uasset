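; AC_PourDose is an action component that pours a selected dose into a cup tool.
; On BeginPlay it caches the owner's AC_Navigation component.
; Start looks up the dose matching the navigation selection, stores its name and pour delay as the action delay, then triggers the action.
; The action function casts the first tool to BP_Cup, adds the dose and emits debug feedback.
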(event `self.ReceiveBeginPlay`
  (`parent.ReceiveBeginPlay`)
  (set `self.Navigation` (`Actor.GetComponentByClass` (`self.GetOwner`) "/Game/Blueprints/Actors/Slots/Navigations/AC_Navigation.AC_Navigation_C")))

(fn `Action_Function`
  ; Action
  (bind _asbp_cup (cast `/Game/Blueprints/Actors/Tools/Instances/BP_Cup` (`self.GetTool` 0)))
  (`/Game/Blueprints/Actors/Tools/Instances/BP_Cup.AddDose` _asbp_cup (`self.Dose`))
  ; FeedBack
  (`/Game/Blueprints/FL_Common.DebugFeedBack` self "Action_Function" true)
  (return))

(fn `Start`
  (returns (Success :type Boolean))
  (if (`self.CanStart`)
    (bind (_success _dose) (`/Game/DataBase/Dose/FL_Dose.GetDose` (cast `/Game/DataBase/Dose/EN_Dose` (`/Game/Blueprints/Actors/Slots/Navigations/AC_Navigation.GetSelected` (`self.Navigation`)))))
    (if _success
      (bind ((`Name_4_F7F5E39D4B7363D308712490117795D8` _name) (`PourDelay_11_A94F8E104A8AD29AA89FC88781EDA1EF` _pourdelay)) (break `/Game/DataBase/Dose/ST_Dose` _dose))
      (set `self.Dose` _name)
      (set `self.ActionDelay` _pourdelay)
      (`self.Action`)
      (return false)
      (else
        _)))
  (return false))