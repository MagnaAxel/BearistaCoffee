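; Slot action that mixes an extra into a cup using two tools, a BP_Extra and a BP_Cup, in either order.
; Start runs the action only if CanStart passes and soft class checks confirm that pairing, returning whether it started.
; ActionFunction tries both orderings through casts, adds the extra's value to the cup and sends the extra actor back to its pool.
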(fn `Action_Function`
  (`|ExecutionSequence`
    (:`then_0`
      (bind _asbp_extra (cast `/Game/Blueprints/Actors/Tools/Instances/BP_Extra` (`self.GetTool` 0)))
      (bind _asbp_cup (cast `/Game/Blueprints/Actors/Tools/Instances/BP_Cup` (`self.GetTool` 1)))
      (`/Game/Blueprints/Actors/Tools/Instances/BP_Cup.AddExtra` _asbp_cup (`/Game/Blueprints/Actors/Tools/Instances/BP_Extra.GetExtra` _asbp_extra))
      (`/Game/Blueprints/Actors/Tools/BP_Tool.ToPool` _asbp_extra)
      (return))
    (:`then_1`
      (bind _asbp_extra_2 (cast `/Game/Blueprints/Actors/Tools/Instances/BP_Extra` (`self.GetTool` 1)))
      (bind _asbp_cup_2 (cast `/Game/Blueprints/Actors/Tools/Instances/BP_Cup` (`self.GetTool` 0)))
      (`/Game/Blueprints/Actors/Tools/Instances/BP_Cup.AddExtra` _asbp_cup_2 (`/Game/Blueprints/Actors/Tools/Instances/BP_Extra.GetExtra` _asbp_extra_2))
      (`/Game/Blueprints/Actors/Tools/BP_Tool.ToPool` _asbp_extra_2)
      (return))))

(fn `Start`
  (returns (Success :type Boolean))
  (if (`self.CanStart`)
    (`KismetSystemLibrary.IsObjectOfSoftClass` (`self.GetTool` 0) "/Game/Blueprints/Actors/Tools/Instances/BP_Extra.BP_Extra_C"
      (:`True`
        (`KismetSystemLibrary.IsObjectOfSoftClass` (`self.GetTool` 1) "/Game/Blueprints/Actors/Tools/Instances/BP_Cup.BP_Cup_C"
          (:`True`
            (`self.Action` :!label _label)
            (return true))
          (:`False`
            _)))
      (:`False`
        (`KismetSystemLibrary.IsObjectOfSoftClass` (`self.GetTool` 0) "/Game/Blueprints/Actors/Tools/Instances/BP_Cup.BP_Cup_C"
          (:`True`
            (`KismetSystemLibrary.IsObjectOfSoftClass` (`self.GetTool` 1) "/Game/Blueprints/Actors/Tools/Instances/BP_Extra.BP_Extra_C"
              (:`True`
                (goto _label))
              (:`False`
                _)))
          (:`False`
            _)))))
  (return false))