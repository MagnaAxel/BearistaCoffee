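; AC_Navigation is a slot navigation actor component that cycles a current Byte through a Bytes array, starting from the first entry on BeginPlay.
; Right and Down events step to the next entry and Left and Up to the previous, wrapping at either end.
; Each step calls the Navigated dispatcher and logs debug feedback, and GetByte exposes the current selection.
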(event `self.ReceiveBeginPlay`
  (set `self.Byte` (`|GetArrayItem` (`self.Bytes`))))

(event `/Game/Blueprints/Actors/Slots/Navigations/IN_Navigation.Right`
  (`self.Next`))

(event `/Game/Blueprints/Actors/Slots/Navigations/IN_Navigation.Down`
  (`self.Next`))

(event `/Game/Blueprints/Actors/Slots/Navigations/IN_Navigation.Left`
  (`self.Previous`))

(event `/Game/Blueprints/Actors/Slots/Navigations/IN_Navigation.Up`
  (`self.Previous`))

(fn `GetByte`
  (returns (Byte :type Byte))
  (return (`self.Byte`)))

(fn `Next`
  ; Action
  (bind _result (`/Engine/EditorBlueprintResources/StandardMacros.IncrementInt` (`KismetArrayLibrary.Array_Find` (`self.Bytes`) (`self.Byte`)))
    (:`  `
      (set `self.Byte` (`|GetArrayItem` (`self.Bytes`) (`KismetMathLibrary.SelectInt` 0 _result (> _result (`KismetArrayLibrary.Array_LastIndex` (`self.Bytes`))))))
      (`self.Navigated`)
      ; FeedBack
      (`/Game/Blueprints/FL_Common.DebugFeedBack` self "Next" true))))

(fn `Previous`
  ; Action
  (bind _result (`/Engine/EditorBlueprintResources/StandardMacros.DecrementInt` (`KismetArrayLibrary.Array_Find` (`self.Bytes`) (`self.Byte`)))
    (:`  `
      (set `self.Byte` (`|GetArrayItem` (`self.Bytes`) (`KismetMathLibrary.SelectInt` (`KismetArrayLibrary.Array_LastIndex` (`self.Bytes`)) _result (< _result 0))))
      (`self.Navigated`)
      ; FeedBack
      (`/Game/Blueprints/FL_Common.DebugFeedBack` self "Previous" true))))