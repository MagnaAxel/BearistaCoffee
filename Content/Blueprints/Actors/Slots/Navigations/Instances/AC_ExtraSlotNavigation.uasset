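; Navigation component for slot actors that applies the navigated selection to extra tools held in the owner's slot.
; On begin play it finds the owner's AC_Slot and binds to both its slotted event and its own navigated event.
; Each trigger, plus an initial call, loops the slot's tools and sets every BP_Extra to the current navigation byte converted to EN_Extra.
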(event `self.ReceiveBeginPlay`
  (`parent.ReceiveBeginPlay`)
  (bind _output_get (set `self.Slot` (`Actor.GetComponentByClass` (`self.GetOwner`) "/Game/Blueprints/Actors/Slots/AC_Slot.AC_Slot_C")))
  (add `/Game/Blueprints/Actors/Slots/AC_Slot.Slotted` _output_get (delegate `Slotted_Event`))
  (add `self.Navigated` (delegate `ApplyExtra`))
  (`self.ApplyExtra`))

(event `Slotted_Event`
  (params (Actor :type "Actor Object Reference"))
  (`self.ApplyExtra`))

(event `ApplyExtra`
  (bind (_keypin _valuepin) (`|MapForEach` (`/Game/Blueprints/Actors/Slots/AC_Slot.Tools` (`self.Slot`)))
    (:`then`
      (bind _asbp_extra (cast `/Game/Blueprints/Actors/Tools/Instances/BP_Extra` _valuepin))
      (`/Game/Blueprints/Actors/Tools/Instances/BP_Extra.SetExtra` _asbp_extra (cast `/Game/DataBase/Extra/EN_Extra` (`self.GetByte`))))))