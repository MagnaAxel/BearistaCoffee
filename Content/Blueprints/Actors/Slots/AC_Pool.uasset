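; AC_Pool is a slot-related component that acts as a pool of tools for refilling a linked SlotActor.
; On BeginPlay it binds RefillSlot to its own slotted event and to the unslotted event of the SlotActor's AC_Slot.
; RefillSlot loops through the Tools map and calls TrySlot for every valid tool, passing the SlotActor and the owning actor, with no early exit.
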(event `self.ReceiveBeginPlay`
  (add `self.Slotted` (delegate `RefillSlot`))
  (add `self.Unslotted` (`Actor.GetComponentByClass` (`self.SlotActor`) "/Game/Blueprints/Actors/Slots/AC_Slot.AC_Slot_C") (delegate `RefillSlot`)))

(event `RefillSlot`
  (params (Actor :type "Actor Object Reference"))
  (bind (_keypin _valuepin) (`|MapForEach` (`self.Tools`))
    (:`then`
      (if (`KismetSystemLibrary.IsValid` _valuepin)
        (`/Game/Blueprints/Actors/Slots/FL_Slot.TrySlot` (`self.SlotActor`) (`self.GetOwner`) _valuepin)))))