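; AC_Slot is an actor component that manages tool slots on its owner, held in a map from slot key to tool actor.
; Each key defines an accepted soft class, relative transform and hidden flag, used to spawn and attach default tools or destroy them.
; Slotting fills a specified or first compatible empty slot through TryCatch, while unslotting detaches the tool and clears its entry.
; Both apply the hidden flag and fire Slotted or Unslotted callbacks.
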(fn `DestroyTools`
  (bind (_keypin _valuepin) (`|MapForEach` (`self.Tools`))
    (:`then`
      (if (`KismetSystemLibrary.IsValid` _valuepin)
        (`Actor.K2_DestroyActor` _valuepin)
        (`BlueprintMapLibrary.Map_Add` (`self.Tools`) _keypin)))))

(fn `GetTool`
  (params (SlotKey :type "/Game/Blueprints/Actors/Slots/ST_SlotKey Structure (by ref)"))
  (returns (Tool :type "Actor Object Reference") (Success :type Boolean))
  (bind _value (`BlueprintMapLibrary.Map_Find` (`self.Tools`) SlotKey))
  (return _value (`KismetSystemLibrary.IsValid` _value)))

(fn `Slot`
  (params (Actor :type "Actor Object Reference") (Tool :type "Actor Object Reference"))
  (returns (Success :type Boolean))
  (bind _keypin (`|MapForEach` (`self.Tools`))
    (:`then`
      (`self.SlotTool` Actor Tool _keypin
        (:`Succeed`
          (return true))))
    (:`CompletedPin`
      (return false))))

(fn `SlotAt`
  (params (Actor :type "Actor Object Reference") (Tool :type "Actor Object Reference") (SlotKey :type "/Game/Blueprints/Actors/Slots/ST_SlotKey Structure"))
  (returns (Success :type Boolean))
  (`self.SlotTool` Actor Tool SlotKey
    (:`Succeed`
      (return true))
    (:`Fail`
      (return false))))

(fn `SpawnTools`
  (bind (_keypin _valuepin) (`|MapForEach` (`self.Tools`))
    (:`then`
      (bind ((`ToolClass_6_A356A8074513D3A00771CC8D2A52FC07` _toolclass) (`RelativeTransform_8_FBE1C6464E6D775494AA2A834BBCCD07` _relativetransform)) (break `/Game/Blueprints/Actors/Slots/ST_SlotKey` _keypin))
      (if (and (not (`KismetSystemLibrary.IsValid` _valuepin)) (`KismetSystemLibrary.IsValidSoftClassReference` _toolclass))
        (bind _returnvalue (`|SpawnActorFromClass` (`|ConvertAsset` _toolclass) (`Actor.GetTransform` (`self.GetOwner`)) "Undefined" "MultiplyWithRoot" null null))
        (`/Game/Blueprints/FL_Common.Attach` _returnvalue (`self.GetOwner`) _relativetransform)
        (if (`.Hidden_10_56A95FC144B7378B0F4141B2F1D62901` (break `/Game/Blueprints/Actors/Slots/ST_SlotKey` _keypin))
          (`Actor.SetActorHiddenInGame` _returnvalue true))
        (`BlueprintMapLibrary.Map_Add` (`self.Tools`) _keypin _returnvalue)))))

(fn `Unslot`
  (params (Actor :type "Actor Object Reference (by ref)") (Tool :type "Actor Object Reference (by ref)"))
  (returns (Success :type Boolean))
  (`self.UnslotTool` Actor Tool
    (:`Succeed`
      (return true))
    (:`Fail`
      (return false))))