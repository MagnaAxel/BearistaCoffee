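; Door interaction component that starts the day in the Bearista coffee game.
; Interact checks the day timer on the Bearista Coffee GSB and calls PlayDay only if that timer handle is not valid.
; On success it restarts the owner's Niagara effect as feedback and returns true, otherwise it returns false.
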(fn `Interact`
  (returns (Success :type Boolean))
  (bind _returnvalue (`Actor.GetComponentByClass` (`self.GetOwner`) "/Script/Niagara.NiagaraComponent"))
  ; Condition
  (if (not (`KismetSystemLibrary.K2_IsValidTimerHandle` (`/Game/Blueprints/Systems/GSB_BearistaCoffee.GetDayTimer` (`/Game/Blueprints/Systems/FL_System.GetGSB_BearistaCoffee`))))
    ; Action
    (`/Game/Blueprints/Systems/GSB_BearistaCoffee.PlayDay` (`/Game/Blueprints/Systems/FL_System.GetGSB_BearistaCoffee`))
    ; FeedBack
    (`NiagaraComponent.ResetSystem` _returnvalue)
    (`self.Activate` _returnvalue false)
    (return true)
    (else
      (return false))))