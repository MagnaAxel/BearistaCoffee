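; AC_Spot is an interactive spot component that holds a Filthy state and can be cleaned.
; Interact succeeds only while the spot is filthy, clearing it through SetFilthy and returning whether it worked.
; SetFilthy stores the value, runs the empty ApplyFilthy hook for visuals or child overrides, fires a ChangedFilthy notification and logs debug feedback.
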(fn `ApplyFilthy`)

(fn `GetFilthy`
  (returns (Filthy :type Boolean))
  (return (`self.Filthy`)))

(fn `Interact`
  (returns (Success :type Boolean))
  ; Condition
  (if (`self.Filthy`)
    ; Action
    (`self.SetFilthy` false)
    ; FeedBack
    (`/Game/Blueprints/FL_Common.DebugFeedBack` self "Interact" true)
    (return true)
    (else
      (`/Game/Blueprints/FL_Common.DebugFeedBack` self "Interact")
      (return false))))

(fn `SetFilthy`
  (params (Filthy :type Boolean))
  ; Action
  (set `self.Filthy` Filthy)
  ; FeedBack
  (`self.ApplyFilthy`)
  (`self.ChangedFilthy`)
  (`/Game/Blueprints/FL_Common.DebugFeedBack` self "SetFilthy" true))