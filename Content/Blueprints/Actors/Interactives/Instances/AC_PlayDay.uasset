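; Actor component for interactives that plays out a timed day when interacted with, counting each day started.
; Interact starts a day only if none is running, setting a timer for the day delay and firing the PlayingDay dispatcher.
; When the timer ends, it clears the handle and fires PlayedDay.
; The timer handle also drives the running-state check and progress percentage queries.
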(event `PlayDay`
  (bind _returnvalue (`KismetSystemLibrary.K2_SetTimerDelegate` (delegate `PlayDay_Event`) (`self.DayDelay`)))
  (set `self.DayTimer` _returnvalue)
  (`/Engine/EditorBlueprintResources/StandardMacros.IncrementInt` (`self.DayCount`)
    (:`  `
      (`self.PlayingDay`))))

(event `PlayDay_Event`
  (`KismetSystemLibrary.K2_ClearAndInvalidateTimerHandle` (`self.DayTimer`))
  (`self.PlayedDay`))

(fn `GetProgression`
  (returns (Progression :type "Float (double-precision)"))
  (bind _daytimer (`self.DayTimer`))
  (if (`KismetSystemLibrary.K2_IsValidTimerHandle` _daytimer)
    (return (`/Game/Blueprints/FL_Common.TimerHandleToPercent` _daytimer))))

(fn `Interact`
  (returns (Success :type Boolean))
  (if (not (`KismetSystemLibrary.K2_IsValidTimerHandle` (`self.DayTimer`)))
    (`self.PlayDay`)
    (return true)))

(fn `IsPlaying`
  (returns (ReturnValue :type Boolean))
  (return (`KismetSystemLibrary.K2_IsValidTimerHandle` (`self.DayTimer`))))