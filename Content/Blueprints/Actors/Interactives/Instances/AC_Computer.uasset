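; AC_Computer is an interactable computer actor in a barista coffee game that opens the computer screen for the player.
; Its Interact override checks the game state's day timer and only succeeds when that timer handle is invalid, so outside a running day.
; On success it switches the player controller's interface to the computer widget and returns true; otherwise it returns false.
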(fn `Interact`
  (returns (Success :type Boolean))
  (bind _interface (`/Game/Blueprints/Systems/Controller/PC_Barista.GetInterface` (`/Game/Blueprints/Systems/FL_System.GetPC_BaristaCoffee` 0)))
  ; Condition
  (if (not (`KismetSystemLibrary.K2_IsValidTimerHandle` (`/Game/Blueprints/Systems/GSB_BearistaCoffee.GetDayTimer` (`/Game/Blueprints/Systems/FL_System.GetGSB_BearistaCoffee`))))
    ; Action
    (`/Game/Blueprints/Widgets/WI_BearistaCoffee.Switch` _interface (`/Game/Blueprints/Widgets/WI_BearistaCoffee.WI_Computer` _interface))
    (return true)
    (else
      (return false))))