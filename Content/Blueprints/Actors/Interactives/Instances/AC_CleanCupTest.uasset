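; AC_CleanCupTest is an interactive actor component that washes cups slotted on its owner, apparently a coffee-game cleaning station.
; Interact gathers cups from keyed AC_Slot slots, hides the interact prompt, starts the acting Niagara effect and sets a timer scaled by cup count.
; When it fires, CleanCups clears and re-slots each cup into CupSlot, switches to the acted effect and calls CleanedCups.
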(event `CleanCups`
  (bind _returnvalue (`Actor.FindComponentByTag` (`self.GetOwner`) "/Script/Niagara.NiagaraComponent" (`self.ActedTag`)))
  (for _array_element (`self.As BP Cup`)
    (`/Game/Blueprints/Actors/Tools/Instances/BP_Cup.Clear` _array_element false)
    (`/Game/Blueprints/Actors/Slots/FL_Slot.TrySlot` (`self.CupSlot`) (`self.GetOwner`) _array_element))
  (`KismetArrayLibrary.Array_Clear` (`self.As BP Cup`))
  (`/Game/Blueprints/FL_Common.DebugFeedBack` self "Action_Function" true)
  (`self.Deactivate` (`Actor.FindComponentByTag` (`self.GetOwner`) "/Script/Niagara.NiagaraComponent" (`self.ActingTag`)))
  (`NiagaraComponent.ResetSystem` _returnvalue)
  (`self.Activate` _returnvalue false)
  (`self.CleanedCups`))

(fn `Interact`
  (params (Actor :type "/Game/Blueprints/Actors/Barista/BP_Barista Object Reference"))
  (returns (Success :type Boolean))
  (locals (CupCount :type Integer) (cups :type Boolean))
  (set `self.Bearista` Actor)
  (for (_array_element _array_index) (`self.Key`)
    (bind _asbp_cup (cast `/Game/Blueprints/Actors/Tools/Instances/BP_Cup` (`/Game/Blueprints/Actors/Slots/AC_Slot.GetTool` (`Actor.GetComponentByClass` (`self.GetOwner`) "/Game/Blueprints/Actors/Slots/AC_Slot.AC_Slot_C") _array_element)))
    (set `local.cups` true)
    (`KismetArrayLibrary.Array_Add` (`self.As BP Cup`) _asbp_cup)
    (bind _result (`/Engine/EditorBlueprintResources/StandardMacros.IncrementInt` _array_index)
      (:`  `
        (set `local.CupCount` _result))))
  (if (`local.cups`)
    (`/Game/Blueprints/Systems/GSB_BearistaCoffee.HideInteract` (`/Game/Blueprints/Systems/FL_System.GetGSB_BearistaCoffee`))
    (`self.Activate` (`Actor.FindComponentByTag` (`self.GetOwner`) "/Script/Niagara.NiagaraComponent" (`self.ActingTag`)) false)
    (`KismetSystemLibrary.K2_SetTimer` null "CleanCups" (`KismetMathLibrary.Conv_IntToDouble` (* (`local.CupCount`) (`self.WashCupTime`))))
    (return true)
    (else
      (return true))))