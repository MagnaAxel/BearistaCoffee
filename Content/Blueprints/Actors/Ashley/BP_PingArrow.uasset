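; BP_PingArrow is an arrow actor that moves itself to a pinged actor when its Ping event is called.
; The event captures its current location as the start and the target's location plus an offset as the end.
; A timeline then interpolates the actor's position between them without sweeping.
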(event `Ping`
  (params (Ping :type "Actor Object Reference"))
  (set `self.End` (+ (`self.K2_GetActorLocation` Ping) (`self.Offset`)))
  (set `self.Start` (`self.K2_GetActorLocation`))
  (bind (_direction _moveto) (`Timeline|MoveToTimeline` :!via `PlayFromStart`)
    (:`Update`
      (`self.K2_SetActorLocation` (`KismetMathLibrary.VLerp` (`self.Start`) (`self.End`) _moveto)))))

(fn `UserConstructionScript`)