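; BP_Ashley is a tutorial guide actor that walks the player through the barista loop once the main menu Play button is clicked.
; Each step pings an arrow at a target and binds to a component event to advance: catch cup, pour, mix extra, catch pastry, serve, clean cup.
; Serving requires two actors attached to the spot and calls Clear on the cup.
; Cleaning destroys the actor, and EndPlay removes the arrow.
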(event `self.ReceiveEndPlay`
  (params (EndPlayReason :type "EEndPlayReason Enum" :default "Destroyed"))
  (`self.K2_DestroyActor` (`self.PingArrow`)))

(event `self.ReceiveBeginPlay`
  (add `/Game/Blueprints/Widgets/Components/WI_Button.OnClicked` (`/Game/Blueprints/Widgets/WI_MainMenu.WI_ButtonPlay` (`/Game/Blueprints/Widgets/WI_BearistaCoffee.WI_MainMenu` (`/Game/Blueprints/Systems/Controller/PC_Barista.GetInterface` (`/Game/Blueprints/Systems/FL_System.GetPC_BaristaCoffee` 0)))) (delegate `OnClicked_Event`)))

(event `OnClicked_Event`
  (`self.LearnCatchCup`))

(event `LearnCatchCup`
  (`/Game/Blueprints/Actors/Ashley/BP_PingArrow.Ping` (`self.PingArrow`) (`self.CupSlot`))
  (add `/Game/Blueprints/Actors/Slots/AC_Slot.Unslotted` (`self.GetComponentByClass` (`self.CupSlot`) "/Game/Blueprints/Actors/Slots/AC_Slot.AC_Slot_C") (delegate `Unslotted_Event`)))

(event `Unslotted_Event`
  (params (Actor :type "Actor Object Reference"))
  (`self.LearnPourDose`))

(event `LearnPourDose`
  (`/Game/Blueprints/Actors/Ashley/BP_PingArrow.Ping` (`self.PingArrow`) (`self.CoffeePotSlot`))
  (add `/Game/Blueprints/Actors/Slots/Actions/AC_Action.Acted` (`self.GetComponentByClass` (`self.CoffeePotSlot`) "/Game/Blueprints/Actors/Slots/Actions/Instances/AC_PourDose.AC_PourDose_C") (delegate `Acted_Event`)))

(event `Acted_Event`
  (`self.LearnMixExtra`))

(event `LearnMixExtra`
  (`/Game/Blueprints/Actors/Ashley/BP_PingArrow.Ping` (`self.PingArrow`) (`self.ExtraSlot`))
  (add `/Game/Blueprints/Actors/Slots/Actions/AC_Action.Acted` (`self.GetComponentByClass` (`GameplayStatics.GetPlayerPawn` 0) "/Game/Blueprints/Actors/Slots/Actions/Instances/AC_MixExtra.AC_MixExtra_C") (delegate `Acted_Event_0`)))

(event `Acted_Event_0`
  (`self.LearnCatchPastrie`))

(event `LearnCatchPastrie`
  (`/Game/Blueprints/Actors/Ashley/BP_PingArrow.Ping` (`self.PingArrow`) (`self.PastrieSlot`))
  (add `/Game/Blueprints/Actors/Slots/AC_Slot.Unslotted` (`self.GetComponentByClass` (`self.PastrieSlot`) "/Game/Blueprints/Actors/Slots/AC_Slot.AC_Slot_C") (delegate `Unslotted_Event_0`)))

(event `Unslotted_Event_0`
  (params (Actor :type "Actor Object Reference"))
  (`self.LearnServeOrder`))

(event `LearnServeOrder`
  (`/Game/Blueprints/Actors/Ashley/BP_PingArrow.Ping` (`self.PingArrow`) (`self.Spot`))
  (add `/Game/Blueprints/Actors/Slots/AC_Slot.Slotted` (`self.GetComponentByClass` (`self.Spot`) "/Game/Blueprints/Actors/Slots/AC_Slot.AC_Slot_C") (delegate `Slotted_Event`)))

(event `Slotted_Event`
  (params (Actor :type "Actor Object Reference"))
  (bind _outactors (`self.GetAttachedActors` (`self.Spot`) true false))
  (if (== (`KismetArrayLibrary.Array_Length` _outactors) 2)
    (for _array_element _outactors
      (bind _asbp_cup (cast `/Game/Blueprints/Actors/Tools/Instances/BP_Cup` _array_element))
      (`/Game/Blueprints/Actors/Tools/Instances/BP_Cup.Clear` _asbp_cup true)
      (`self.LearnCleanCup`))))

(event `LearnCleanCup`
  (`/Game/Blueprints/Actors/Ashley/BP_PingArrow.Ping` (`self.PingArrow`) (`self.SinkSlot`))
  (add `/Game/Blueprints/Actors/Slots/Actions/AC_Action.Acted` (`self.GetComponentByClass` (`self.SinkSlot`) "/Game/Blueprints/Actors/Slots/Actions/Instances/AC_CleanCup.AC_CleanCup_C") (delegate `Acted_Event_1`)))

(event `Acted_Event_1`
  (`self.K2_DestroyActor`))

(fn `UserConstructionScript`)