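; PC_Barista is a player controller that sets up input, camera and game UI on BeginPlay.
; It adds the gamepad Enhanced Input mapping context, sets the view target to a CameraActor found in the level, then creates WI_Game and adds it to the viewport.
; GetInterface returns the Interface variable, which BeginPlay sets to None rather than to the created widget.
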(event `self.ReceiveBeginPlay`
  (`|ExecutionSequence`
    (:`then_0`
      (`EnhancedInputSubsystemInterface.AddMappingContext` (subsystem `EnhancedInputLocalPlayerSubsystem`) "/Game/Blueprints/Systems/Controller/InputMaps/IMC_GamePad.IMC_GamePad" 0 (struct)))
    (:`then_1`
      (bind _returnvalue (`GameplayStatics.GetActorOfClass` "/Script/Engine.CameraActor"))
      (`self.SetViewTargetWithBlend` _returnvalue))
    (:`then_2`
      (bind _returnvalue_2 (`|CreateWidget` "/Game/Blueprints/Widgets/Pages/WI_Game.WI_Game_C" self))
      (set `self.Interface` null)
      (`UserWidget.AddToViewport` _returnvalue_2 0))))

(fn `GetInterface`
  (returns (Interface :type "/Game/Blueprints/Widgets/WI_BearistaCoffee Object Reference"))
  (return (`self.Interface`)))

(fn `UserConstructionScript`)