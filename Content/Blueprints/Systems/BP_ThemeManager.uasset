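; BP_ThemeManager applies the current visual theme to the environment, lighting and ground.
; It follows theme changes from GSBBearistaCoffee, syncing on BeginPlay, and also applies its own theme in the construction script.
; Each theme resolves to a row that supplies a level, light color and ground color.
; It swaps environments by unloading and streaming soft-referenced levels, then tints a rect light and the ground mesh's "Color" material parameter.
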(event `self.ReceiveBeginPlay`
  (add `/Game/Blueprints/Systems/GSB_BearistaCoffee.ChangedTheme` (`/Game/Blueprints/Systems/FL_System.GetGSB_BearistaCoffee`) (delegate `ChangedTheme_Event`))
  (`self.ChangedTheme_Event`))

(event `ChangedTheme_Event`
  (`self.SetTheme` (`/Game/Blueprints/Systems/GSB_BearistaCoffee.GetTheme` (`/Game/Blueprints/Systems/FL_System.GetGSB_BearistaCoffee`))))

(event `ApplyEnvironment`
  (params (Level :type "World Soft Object Reference"))
  (`GameplayStatics.UnloadStreamLevelBySoftObjectPtr` (`self.Environment`) true)
  (`GameplayStatics.LoadStreamLevelBySoftObjectPtr` Level true)
  (set `self.Environment` Level))

(fn `ApplyGround`
  (params (Ground :type "LinearColor Structure"))
  (`MeshComponent.SetColorParameterValueOnMaterials` (`StaticMeshActor.StaticMeshComponent` (`self.Ground`)) "Color" Ground))

(fn `ApplyLight`
  (params (Light :type "LinearColor Structure"))
  (`LightComponent.SetLightColor` (`RectLight.RectLightComponent` (`self.Light`)) Light true))

(fn `ApplyTheme`
  (bind (_success _out_row) (`/Game/DataBase/Theme/FL_Theme.GetTheme` (`self.Theme`)))
  (if _success
    (`|ExecutionSequence`
      (:`then_0`
        (bind ((`Environment_3_AB5858524701154F1F8E44870DCED209` _environment) (`Light_12_06B459714938E80BC728A89FC5256C2D` _light) (`Ground_14_CE0960A643DBFFAA2B08DD9B1D435783` _ground)) (break `/Game/DataBase/Theme/ST_Theme` _out_row))
        (`self.ApplyEnvironment` (`.WorldAsset` (break `SoftWorldReference` _environment))))
      (:`then_1`
        (`self.ApplyLight` _light))
      (:`then_2`
        (`self.ApplyGround` _ground)))))

(fn `GetTheme`
  (returns (Theme :type "/Game/DataBase/Theme/EN_Theme Enum"))
  (return (`self.Theme`)))

(fn `SetTheme`
  (params (Theme :type "/Game/DataBase/Theme/EN_Theme Enum" :default "NewEnumerator0"))
  (set `self.Theme` Theme)
  (`self.ApplyTheme`))

(fn `UserConstructionScript`
  (`self.ApplyTheme`))