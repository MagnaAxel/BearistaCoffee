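; BP_AssetManager applies themed static meshes to groups of mesh components, keeping each asset's theme in sync with GSBBearistaCoffee.
; Its Assets map stores a theme and component list per asset, which the construction script applies.
; On BeginPlay and each change notification, it updates only assets whose theme differs from GSBBearistaCoffee.
; Each update looks up the mesh by asset and theme, loads it synchronously and sets it on every listed component.
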(event `self.ReceiveBeginPlay`
  (add `/Game/Blueprints/Systems/GSB_BearistaCoffee.ChangedAsset` (`/Game/Blueprints/Systems/FL_System.GetGSB_BearistaCoffee`) (delegate `ChangedAsset_Event`))
  (`self.ChangedAsset_Event`))

(event `ChangedAsset_Event`
  (bind (_keypin _valuepin) (`|MapForEach` (`self.Assets`))
    (:`then`
      (bind _theme (`/Game/Blueprints/Systems/GSB_BearistaCoffee.GetAsset` (`/Game/Blueprints/Systems/FL_System.GetGSB_BearistaCoffee`) _keypin))
      (if (`|EnumInequality` _theme (`.Theme_3_7530A88E412D9177D0B6B0A63BAC75A0` (break `/Game/Blueprints/Systems/ST_AssetValue` _valuepin)))
        (`self.SetAsset` _keypin _theme)))))

(fn `ApplyAsset`
  (params (Asset :type "/Game/DataBase/Asset/EN_Asset Enum" :default "NewEnumerator0") (Theme :type "/Game/DataBase/Asset/EN_Theme Enum" :default "NewEnumerator0"))
  (bind (_success _asset) (`/Game/DataBase/Asset/FL_Asset.GetAsset` Asset Theme))
  (bind _returnvalue (`KismetSystemLibrary.LoadAsset_Blocking` (`.StaticMesh_5_B9DD2A284917C3A7D4A907A63F22F040` (break `/Game/DataBase/Asset/ST_Asset` _asset))))
  (bind _asstatic_mesh (cast `StaticMesh` _returnvalue))
  (for _array_element (`.Meshs_6_A007C6B24CA30D3B199423AA311A2EB2` (break `/Game/Blueprints/Systems/ST_AssetValue` (`BlueprintMapLibrary.Map_Find` (`self.Assets`) Asset)))
    (`StaticMeshComponent.SetStaticMesh` (`StaticMeshActor.StaticMeshComponent` _array_element) _asstatic_mesh)))

(fn `ApplyAssets`
  (bind (_keypin _valuepin) (`|MapForEach` (`self.Assets`))
    (:`then`
      (`self.ApplyAsset` _keypin (`.Theme_3_7530A88E412D9177D0B6B0A63BAC75A0` (break `/Game/Blueprints/Systems/ST_AssetValue` _valuepin))))))

(fn `SetAsset`
  (params (Asset :type "/Game/DataBase/Asset/EN_Asset Enum" :default "NewEnumerator0") (Theme :type "/Game/DataBase/Asset/EN_Theme Enum" :default "NewEnumerator0"))
  (bind _structout (setmembers `/Game/Blueprints/Systems/ST_AssetValue` :`StructRef` (`BlueprintMapLibrary.Map_Find` (`self.Assets`) Asset) :`Theme` Theme))
  (`BlueprintMapLibrary.Map_Add` (`self.Assets`) Asset _structout)
  (`self.ApplyAsset` Asset Theme))

(fn `UserConstructionScript`
  (`self.ApplyAssets`))