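; FL_System is a helper library of typed getters for the Bearista Coffee game's core framework objects.
; It returns the game mode as GMB_BearistaCoffee, the game state as GSB_BearistaCoffee, and the player controller at a given index as PC_Barista.
; Each getter wraps the engine lookup in a cast and stops without returning the object if the cast fails.
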(fn `GetGMB_BearistaCoffee`
  (returns (GMB :type "/Game/Blueprints/Systems/GMB_BearistaCoffee Object Reference"))
  (bind _asgmb_bearista_coffee (cast `/Game/Blueprints/Systems/GMB_BearistaCoffee` (`GameplayStatics.GetGameMode` null)))
  (return _asgmb_bearista_coffee))

(fn `GetGSB_BearistaCoffee`
  (returns (GSB :type "/Game/Blueprints/Systems/GSB_BearistaCoffee Object Reference"))
  (bind _asgsb_bearista_coffee (cast `/Game/Blueprints/Systems/GSB_BearistaCoffee` (`GameplayStatics.GetGameState` null)))
  (return _asgsb_bearista_coffee))

(fn `GetPC_BaristaCoffee`
  (params (PlayerIndex :type Integer))
  (returns (`PC Barista` :type "/Game/Blueprints/Systems/Controller/PC_Barista Object Reference"))
  (bind _aspc_barista (cast `/Game/Blueprints/Systems/Controller/PC_Barista` (`GameplayStatics.GetPlayerController` null PlayerIndex)))
  (return _aspc_barista))