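; Game state for Bearista Coffee that owns player progress: popularity, Pawies, client affinities, difficulty, day, asset themes, progression and inventory.
; BeginPlay loads or creates the SaveGame, then reapplies most values; Save writes it to its slot.
; Setters update the data and call Apply functions that broadcast changes, resolving popularity and service tiers into data.
; Service level stays outside the save, and PlayDay increments the day and runs a timer announcing its end.
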(event `self.ReceiveBeginPlay`
  (`self.Load`))

(event `PlayDay`
  (bind _returnvalue (`KismetSystemLibrary.K2_SetTimerDelegate` (delegate `PlayDay_Event`) (`self.DayDelay`)))
  (set `self.DayTimer` _returnvalue)
  (`self.AddDay` 1)
  (`self.PlayingDay`))

(event `PlayDay_Event`
  (`KismetSystemLibrary.K2_ClearAndInvalidateTimerHandle` (`self.DayTimer`))
  (`self.PlayedDay`))

(fn `AddAffinity`
  (params (Client :type "/Game/DataBase/Client/EN_Client Enum (by ref)") (Affinity :type Integer))
  (`BlueprintMapLibrary.Map_Add` (`/Game/Blueprints/Systems/SG_BearistaCoffee.Affinities` (`self.SaveGame`)) Client (+ (`BlueprintMapLibrary.Map_Find` (`/Game/Blueprints/Systems/SG_BearistaCoffee.Affinities` (`self.SaveGame`)) Client) Affinity))
  (`self.ApplyAffinity`))

(fn `AddDay`
  (params (Day :type Integer))
  (set `/Game/Blueprints/Systems/SG_BearistaCoffee.Day` (`KismetMathLibrary.Max` (+ (`/Game/Blueprints/Systems/SG_BearistaCoffee.Day` (`self.SaveGame`)) Day)) (`self.SaveGame`))
  (`self.ApplyDay`))

(fn `AddInventory`
  (params (Asset :type "/Game/DataBase/Asset/ST_Asset Structure (by ref)"))
  (`KismetArrayLibrary.Array_AddUnique` (`/Game/Blueprints/Systems/SG_BearistaCoffee.Inventory` (`self.SaveGame`)) Asset)
  (`self.ChangedInventory`))

(fn `AddPawies`
  (params (Pawies :type Integer))
  (set `/Game/Blueprints/Systems/SG_BearistaCoffee.Pawies` (`KismetMathLibrary.Max` (+ (`/Game/Blueprints/Systems/SG_BearistaCoffee.Pawies` (`self.SaveGame`)) Pawies)) (`self.SaveGame`))
  (`self.ApplyPawies`))

(fn `AddPopularity`
  (params (Popularity :type Integer))
  (set `/Game/Blueprints/Systems/SG_BearistaCoffee.Popularity` (`KismetMathLibrary.Clamp` (+ (`/Game/Blueprints/Systems/SG_BearistaCoffee.Popularity` (`self.SaveGame`)) Popularity) 0 (`self.PopularityMax`)) (`self.SaveGame`))
  (`self.ApplyPopularity`))

(fn `AddProgression`
  (params (Progression :type "/Game/DataBase/Story/EN_Story Enum (by ref)"))
  (`KismetArrayLibrary.Array_AddUnique` (`/Game/Blueprints/Systems/SG_BearistaCoffee.Progression` (`self.SaveGame`)) Progression)
  (`self.ApplyProgression`))

(fn `AddService`
  (params (Service :type Integer))
  (set `self.ServiceIndex` (`KismetMathLibrary.Clamp` (+ (`self.ServiceIndex`) Service) (`self.ServiceMin`) (`self.ServiceMax`)))
  (`self.ApplyService`))

(fn `ApplyAffinity`
  (`self.AddedAffinity`))

(fn `ApplyAsset`
  (`self.ChangedAsset`))

(fn `ApplyDay`
  (`self.ChangedDay`))

(fn `ApplyDifficulty`
  (`self.ChangedDifficulty`))

(fn `ApplyInventory`
  (`self.ChangedInventory`))

(fn `ApplyPawies`
  (`self.AddedPawies`))

(fn `ApplyPopularity`
  (bind (_success _popularity) (`/Game/DataBase/Popularity/FL_Popularity.GetPopularity` (`/Game/Blueprints/Systems/SG_BearistaCoffee.Popularity` (`self.SaveGame`))))
  (set `self.PopularityData` _popularity)
  (`self.AddedPopularity`))

(fn `ApplyProgression`
  (`self.ChangedProgression`))

(fn `ApplyService`
  (bind (_success _service) (`/Game/DataBase/Service/FL_Service.GetService` (`self.ServiceIndex`)))
  (set `self.ServiceData` _service)
  (`self.AddedService`))

(fn `GetAffinity`
  (params (Client :type "/Game/DataBase/Client/EN_Client Enum" :default "NewEnumerator0"))
  (returns (Affinity :type Integer))
  (return (`BlueprintMapLibrary.Map_Find` (`/Game/Blueprints/Systems/SG_BearistaCoffee.Affinities` (`self.SaveGame`)) Client)))

(fn `GetAsset`
  (params (Asset :type "/Game/DataBase/Asset/EN_Asset Enum (by ref)"))
  (returns (Theme :type "/Game/DataBase/Asset/EN_Theme Enum"))
  (return (`BlueprintMapLibrary.Map_Find` (`/Game/Blueprints/Systems/SG_BearistaCoffee.Assets` (`self.SaveGame`)) Asset)))

(fn `GetDay`
  (returns (Day :type Integer))
  (return (`/Game/Blueprints/Systems/SG_BearistaCoffee.Day` (`self.SaveGame`))))

(fn `GetDayTimer`
  (returns (DayTimer :type "TimerHandle Structure"))
  (return (`self.DayTimer`)))

(fn `GetDifficultyData`
  (returns (Difficulty :type "/Game/DataBase/Difficulty/ST_Difficulty Structure"))
  (bind (_success _difficulty) (`/Game/DataBase/Difficulty/FL_Difficulty.GetDifficulty` (`/Game/Blueprints/Systems/SG_BearistaCoffee.Difficulty` (`self.SaveGame`))))
  (return _difficulty))

(fn `GetInventory`
  (returns (Inventory :type "Array of /Game/DataBase/Asset/ST_Asset Structure"))
  (return (`/Game/Blueprints/Systems/SG_BearistaCoffee.Inventory` (`self.SaveGame`))))

(fn `GetPawies`
  (returns (Pawies :type Integer))
  (return (`/Game/Blueprints/Systems/SG_BearistaCoffee.Pawies` (`self.SaveGame`))))

(fn `GetPopularityData`
  (returns (PopularityData :type "/Game/DataBase/Popularity/ST_Popularity Structure"))
  (return (`self.PopularityData`)))

(fn `GetPopularityValue`
  (returns (Popularity :type Integer))
  (return (`/Game/Blueprints/Systems/SG_BearistaCoffee.Popularity` (`self.SaveGame`))))

(fn `GetProgression`
  (returns (Progression :type "Array of /Game/DataBase/Story/EN_Story Enum"))
  (return (`/Game/Blueprints/Systems/SG_BearistaCoffee.Progression` (`self.SaveGame`))))

(fn `GetServiceData`
  (returns (ServiceData :type "/Game/DataBase/Service/ST_Service Structure"))
  (return (`self.ServiceData`)))

(fn `GetServiceValue`
  (returns (ServiceValue :type Integer))
  (return (`self.ServiceIndex`)))

(fn `Load`
  (`|ExecutionSequence`
    (:`then_0`
      (bind _returnvalue (`GameplayStatics.DoesSaveGameExist` (`self.SlotName`)))
      (if _returnvalue
        (bind _returnvalue_2 (`GameplayStatics.LoadGameFromSlot` (`self.SlotName`)))
        (bind _assg_bearista_coffee (cast `/Game/Blueprints/Systems/SG_BearistaCoffee` _returnvalue_2))
        (set `self.SaveGame` _assg_bearista_coffee)
        (else
          (bind _returnvalue_3 (`|GenericCreateObject` "/Game/Blueprints/Systems/SG_BearistaCoffee.SG_BearistaCoffee_C"))
          (set `self.SaveGame` _returnvalue_3))))
    (:`then_1`
      (`self.ApplyPopularity`)
      (`self.ApplyPawies`)
      (`self.ApplyAffinity`)
      (`self.ApplyDay`)
      (`self.ApplyAsset`)
      (`self.ApplyDifficulty`))))

(fn `ResetService`
  (set `self.ServiceIndex` 1)
  (`self.ApplyService`)
  (`self.ResetedService`))

(fn `Save`
  (bind _returnvalue (`GameplayStatics.SaveGameToSlot` (`self.SaveGame`) (`self.SlotName`)))
  (`KismetSystemLibrary.PrintString` (`KismetStringLibrary.Conv_BoolToString` _returnvalue)))

(fn `SetAsset`
  (params (Asset :type "/Game/DataBase/Asset/EN_Asset Enum" :default "NewEnumerator0") (Theme :type "/Game/DataBase/Asset/EN_Theme Enum" :default "NewEnumerator0"))
  (`BlueprintMapLibrary.Map_Add` (`/Game/Blueprints/Systems/SG_BearistaCoffee.Assets` (`self.SaveGame`)) Asset Theme)
  (`self.ApplyAsset`))

(fn `SetDifficulty`
  (params (Difficulty :type "/Game/DataBase/Difficulty/EN_Difficulty Enum" :default "NewEnumerator0"))
  (set `/Game/Blueprints/Systems/SG_BearistaCoffee.Difficulty` Difficulty (`self.SaveGame`))
  (`self.ApplyDifficulty`))

(fn `UserConstructionScript`)