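; Light manager for the Bearista Coffee game that drives time-of-day and seasonal lighting.
; During the playing day it polls the day timer every tick, using its progress to lerp sun and light-ray rotation and color from day to night.
; SeasonIndex selects the palettes, with ground and bar-light colors applied only in the construction script.
; SetSeasonIndex is empty, and winter ground mistakenly uses the autumn bar color.
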(event `self.ReceiveBeginPlay`
  (add `/Game/Blueprints/Systems/GSB_BearistaCoffee.PlayingDay` (`/Game/Blueprints/Systems/FL_System.GetGSB_BearistaCoffee`) (delegate `PlayingDay_Event`)))

(event `PlayingDay_Event`
  (if (`KismetSystemLibrary.K2_IsValidTimerHandle` (`/Game/Blueprints/Systems/GSB_BearistaCoffee.GetDayTimer` (`/Game/Blueprints/Systems/FL_System.GetGSB_BearistaCoffee`))) :!label _label
    (`self.SetDayAlpha` (`/Game/Blueprints/FL_Common.TimerHandleToPercent` (`/Game/Blueprints/Systems/GSB_BearistaCoffee.GetDayTimer` (`/Game/Blueprints/Systems/FL_System.GetGSB_BearistaCoffee`))))
    (`KismetSystemLibrary.DelayUntilNextTick`)
    (goto _label)))

(fn `ApplyDayAlpha`
  (`self.K2_SetActorRotation` (`self.SunLight`) (`self.GetTimeRotation`) false)
  (`self.K2_SetActorRotation` (`self.LightRay`) (`KismetMathLibrary.ComposeRotators` (`self.GetTimeRotation`) (`self.LightRayOffset`)) false)
  (`LightComponent.SetLightColor` (`Light.LightComponent` (`self.SunLight`)) (`self.GetTimeColor`) true)
  (`MeshComponent.SetColorParameterValueOnMaterials` (`StaticMeshActor.StaticMeshComponent` (`self.LightRay`)) "Color" (`self.GetTimeColor`)))

(fn `ApplySeasonIndex`
  (`MeshComponent.SetColorParameterValueOnMaterials` (`StaticMeshActor.StaticMeshComponent` (`self.GroundPlane`)) "Color" (`self.GetGroundColor`))
  (for _array_element (`self.BarLight`)
    (`LightComponent.SetLightColor` (`RectLight.RectLightComponent` _array_element) (`self.GetBarColor`) true)))

(fn `GetBarColor`
  (returns (BarColor :type "LinearColor Structure"))
  (return (select `int` (`self.SeasonIndex`) :`0` (`self.SpringColorBar`) :`1` (`self.SummerColorBar`) :`2` (`self.AutmnColorBar`) :`3` (`self.WinterColorBar`))))

(fn `GetGroundColor`
  (returns (`Ground Color` :type "LinearColor Structure"))
  (return (select `int` (`self.SeasonIndex`) :`0` (`self.SpringColorGround`) :`1` (`self.SummerColorGround`) :`2` (`self.AutmnColorGround`) :`3` (`self.AutmnColorBar`))))

(fn `GetTimeColor`
  (returns (TimeColor :type "LinearColor Structure"))
  (return (`KismetMathLibrary.LinearColorLerp` (select `int` (`self.SeasonIndex`) :`0` (`self.SpringColorDay`) :`1` (`self.SummerColorDay`) :`2` (`self.AutumnColorDay`) :`3` (`self.WinterColorDay`)) (select `int` (`self.SeasonIndex`) :`0` (`self.SpringColorNight`) :`1` (`self.SummerColorNight`) :`2` (`self.AutumnColorNight`) :`3` (`self.WinterColorNight`)) (`self.DayAlpha`))))

(fn `GetTimeRotation`
  (returns (TimeRotation :type "Rotator Structure"))
  (return (`KismetMathLibrary.RLerp` (`self.DayRotation`) (`self.NightRotation`) (`self.DayAlpha`) true)))

(fn `SetDayAlpha`
  (params (Alpha :type "Float (double-precision)"))
  (set `self.DayAlpha` Alpha)
  (`self.ApplyDayAlpha`))

(fn `SetSeasonIndex`)

(fn `UserConstructionScript`
  (`self.ApplyDayAlpha`)
  (`self.ApplySeasonIndex`))