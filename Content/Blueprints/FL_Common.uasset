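; Blueprint function library of shared gameplay helpers for tracing, attachment, interface lookup, timer progress, spline sampling and debug printing.
; FindStatic and FindTool line-trace along an actor's forward vector on separate channels, with debug drawing, using LineTraceVectors for endpoints.
; FindInterface and FindInterfaces search both the actor and its components for implementers.
; IsCompatible treats an invalid soft class reference as a match, and GetSplineTransformAt maps clamped alpha to world-space spline distance.
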(fn `Attach`
  (params (Target :type "Actor Object Reference") (ParentActor :type "Actor Object Reference") (RelativeTransform :type "Transform Structure"))
  (`Actor.K2_AttachToActor` Target ParentActor "None" "KeepRelative" "KeepRelative" "KeepWorld" false)
  (`Actor.K2_SetActorRelativeTransform` Target RelativeTransform false false))

(fn `DebugFeedBack`
  (params (Object :type "Object Object Reference") (Action :type String) (Success :type Boolean))
  (`KismetSystemLibrary.PrintString` null (`KismetStringLibrary.Concat_StrStr` (`KismetSystemLibrary.GetDisplayName` Object) ": " Action "-> " (`KismetMathLibrary.SelectString` "Succeed" "Fail" Success))))

(fn `FindInterface`
  (params (Actor :type "Actor Object Reference") (Interface :type "Interface Class Reference"))
  (returns (Success :type Boolean) (Object :type "Object Object Reference"))
  (bind _returnvalue (`Actor.GetComponentsByInterface` Actor Interface))
  (if (`KismetSystemLibrary.IsValid` Actor)
    (`|ExecutionSequence`
      (:`then_0`
        (if (`KismetSystemLibrary.DoesImplementInterface` Actor Interface)
          (return true Actor)))
      (:`then_1`
        (if (`KismetArrayLibrary.Array_IsNotEmpty` _returnvalue)
          (return true (`|GetArrayItem` _returnvalue)))))
    (else
      (return false null))))

(fn `FindInterfaces`
  (params (Actor :type "Actor Object Reference") (Interface :type "Interface Class Reference"))
  (returns (Success :type Boolean) (Objects :type "Array of Object Object Reference"))
  (locals (LocalObjects :type "Array of Object Object Reference"))
  (bind _localobjects (`local.LocalObjects`))
  (if (`KismetSystemLibrary.IsValid` Actor)
    (`|ExecutionSequence`
      (:`then_0`
        (if (`KismetSystemLibrary.DoesImplementInterface` Actor Interface)
          (`KismetArrayLibrary.Array_Add` (`local.LocalObjects`) Actor)))
      (:`then_1`
        (`KismetArrayLibrary.Array_Append` (`local.LocalObjects`) (`Actor.GetComponentsByInterface` Actor Interface)))
      (:`then_2`
        (return (`KismetArrayLibrary.Array_IsNotEmpty` _localobjects) _localobjects)))
    (else
      (return false))))

(fn `FindStatic`
  (params (Target :type "Actor Object Reference") (Range :type Integer))
  (returns (Success :type Boolean) (Static :type "Actor Object Reference"))
  (bind (_start _end) (`self.LineTraceVectors` Target Range))
  (bind (_outhit _returnvalue) (`KismetSystemLibrary.LineTraceSingle` :`Start` _start :`End` _end :`TraceChannel` "TraceTypeQuery4" :`DrawDebugType` "ForDuration" :`DrawTime` 1.0))
  (return _returnvalue (`.HitActor` (`GameplayStatics.BreakHitResult` _outhit))))

(fn `FindTool`
  (params (Target :type "Actor Object Reference") (Range :type Integer) (ActorsToIgnore :type "Array of Actor Object Reference (by ref)"))
  (returns (Success :type Boolean) (Tool :type "Actor Object Reference"))
  (bind (_start _end) (`self.LineTraceVectors` Target Range))
  (bind (_outhit _returnvalue) (`KismetSystemLibrary.LineTraceSingle` null _start _end "TraceTypeQuery3" false ActorsToIgnore "ForDuration" true (struct :`R` 1.0 :`A` 1.0) (struct :`G` 1.0 :`A` 1.0) 1.0))
  (return _returnvalue (`.HitActor` (`GameplayStatics.BreakHitResult` _outhit))))

(fn `GetSplineTransformAt`
  (params (Spline :type "SplineComponent Object Reference") (Alpha :type "Float (double-precision)") (Rotation :type "Rotator Structure"))
  (returns (Transform :type "Transform Structure"))
  (bind (_returnvalue_location _returnvalue_rotation _returnvalue_scale) (`KismetMathLibrary.BreakTransform` (`SplineComponent.GetTransformAtDistanceAlongSpline` Spline (`KismetMathLibrary.Lerp` 0.0 (`SplineComponent.GetSplineLength` Spline) (`KismetMathLibrary.FClamp` Alpha)) "World" false)))
  (return (`KismetMathLibrary.MakeTransform` _returnvalue_location (`KismetMathLibrary.ComposeRotators` _returnvalue_rotation Rotation) _returnvalue_scale)))

(fn `IsCompatible`
  (params (SoftObjectClass :type "Object Soft Class Reference (by ref)") (Object :type "Object Object Reference"))
  (returns (Success :type Boolean))
  (if (`KismetSystemLibrary.IsValidSoftClassReference` SoftObjectClass)
    (`KismetSystemLibrary.IsObjectOfSoftClass` Object SoftObjectClass
      (:`True`
        _)
      (:`False`
        (return false))))
  (return true))

(fn `LineTraceVectors`
  (params (Target :type "Actor Object Reference") (Range :type Integer))
  (returns (Start :type "Vector Structure") (End :type "Vector Structure"))
  (bind _returnvalue (`Actor.K2_GetActorLocation` Target))
  (return _returnvalue (+ _returnvalue (* (`Actor.GetActorForwardVector` Target) Range))))

(fn `TimerHandleToPercent`
  (params (TimerHandle :type "TimerHandle Structure (by ref)") (Reversed :type Boolean))
  (returns (Percent :type "Float (double-precision)"))
  (return (/ (`KismetMathLibrary.SelectFloat` (`KismetSystemLibrary.K2_GetTimerRemainingTimeHandle` null TimerHandle) (`KismetSystemLibrary.K2_GetTimerElapsedTimeHandle` null TimerHandle) Reversed) (+ (`KismetSystemLibrary.K2_GetTimerRemainingTimeHandle` null TimerHandle) (`KismetSystemLibrary.K2_GetTimerElapsedTimeHandle` null TimerHandle)))))